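; Player controller for the Loadout phase that shows the mouse cursor and links team selection to the game state and HUD.
; RequestTeam passes the team, index and PlayerState to BP_GS_Loaout for handling.
; Blue, red and spectator team updates are relayed to BP_HUD_Loadout through a lazily cached reference.
; Outfit and weapon requests are empty stubs.
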(event `self.ReceiveBeginPlay`
  (`|ExecutionSequence`
    (:`then_0`
      (`self.bShowDebug`
        (:`then`
          (`KismetSystemLibrary.PrintString` "BP_PC_Loadout - EVENT Begin Play" true true (struct :`G` 0.66 :`B` 1.0 :`A` 1.0) 3.0))
        (:`else`)))
    (:`then_1`
      (set `self.bShowMouseCursor` true))))

(event `HUDStart`
  (`|ExecutionSequence`
    (:`then_0`
      (`self.bShowDebug`
        (:`then`
          (`KismetSystemLibrary.PrintString` "BP_PC_Loadout - EVENT HUD Start" true true (struct :`G` 0.66 :`B` 1.0 :`A` 1.0) 3.0))
        (:`else`)))
    (:`then_1`
      (set `self.bShowMouseCursor` true))
    (:`then_2`
      (`self.As BP HUD Loadout`
        (:`then`)
        (:`else`
          (bind _asbp_hud_loadout (cast `/Game/AIPhases/Loadout/HUD/BP_HUD_Loadout` (`self.GetHUD`)))
          (set `self.As BP HUD Loadout` _asbp_hud_loadout))))))

(event `RequestTeam`
  (params (Team :type "/Game/AIPhases/Blueprints/Team/Enum/E_Team Enum" :default "NewEnumerator0") (Index :type Integer))
  (`|ExecutionSequence`
    (:`then_0`
      (`self.bShowDebug`
        (:`then`
          (`KismetSystemLibrary.PrintString` "BP_PC_CustomLobby - EVENT Client Refresh Team Blue" true true (struct :`G` 0.66 :`B` 1.0 :`A` 1.0) 3.0))
        (:`else`)))
    (:`then_1`
      (bind _asbp_gs_loaout (cast `/Game/AIPhases/Loadout/Modes/BP_GS_Loaout` (`GameplayStatics.GetGameState`)))
      (`/Game/AIPhases/Loadout/Modes/BP_GS_Loaout.HandleTeamRequest` _asbp_gs_loaout Team Index (`self.PlayerState`)))))

(event `HUDTeamBlueUpdate`
  (params (BlueTeam :type "Array of PlayerState Object Reference"))
  (`|ExecutionSequence`
    (:`then_0`
      (`self.bShowDebug`
        (:`then`
          (`KismetSystemLibrary.PrintString` "BP_PC_CustomLobby - EVENT Client Refresh Team Blue" true true (struct :`G` 0.66 :`B` 1.0 :`A` 1.0) 3.0))
        (:`else`)))
    (:`then_1`
      (`self.As BP HUD Loadout`
        (:`then`
          _)
        (:`else`
          (bind _asbp_hud_loadout (cast `/Game/AIPhases/Loadout/HUD/BP_HUD_Loadout` (`self.GetHUD`)))
          (set `self.As BP HUD Loadout` _asbp_hud_loadout)))
      (`/Game/AIPhases/Loadout/HUD/BP_HUD_Loadout.TeamBlueUpdate` (`self.As BP HUD Loadout`) BlueTeam))))

(event `HUDTeamRedUpdate`
  (params (TeamRed :type "Array of PlayerState Object Reference"))
  (`|ExecutionSequence`
    (:`then_0`
      (`self.bShowDebug`
        (:`then`
          (`KismetSystemLibrary.PrintString` "BP_PC_CustomLobby - EVENT Client Refresh Team Red" true true (struct :`G` 0.66 :`B` 1.0 :`A` 1.0) 3.0))
        (:`else`)))
    (:`then_1`
      (`self.As BP HUD Loadout`
        (:`then`
          _)
        (:`else`
          (bind _asbp_hud_loadout (cast `/Game/AIPhases/Loadout/HUD/BP_HUD_Loadout` (`self.GetHUD`)))
          (set `self.As BP HUD Loadout` _asbp_hud_loadout)))
      (`/Game/AIPhases/Loadout/HUD/BP_HUD_Loadout.TeamRedUpdate` (`self.As BP HUD Loadout`) TeamRed))))

(event `HUDTeamSpectatorUpdate`
  (params (TeamSpectator :type "Array of PlayerState Object Reference"))
  (`|ExecutionSequence`
    (:`then_0`
      (`self.bShowDebug`
        (:`then`
          (`KismetSystemLibrary.PrintString` "BP_PC_CustomLobby - EVENT Client Refresh Team Spectator" true true (struct :`G` 0.66 :`B` 1.0 :`A` 1.0) 3.0))
        (:`else`)))
    (:`then_1`
      (`self.As BP HUD Loadout`
        (:`then`
          _)
        (:`else`
          (bind _asbp_hud_loadout (cast `/Game/AIPhases/Loadout/HUD/BP_HUD_Loadout` (`self.GetHUD`)))
          (set `self.As BP HUD Loadout` _asbp_hud_loadout)))
      (`/Game/AIPhases/Loadout/HUD/BP_HUD_Loadout.TeamSpectatorUpdate` (`self.As BP HUD Loadout`) TeamSpectator))))

(event `RequestOutfit`
  (params (Outfit :type "SkeletalMesh Object Reference")))

(event `RequestWeapon`
  (params (WeaponData :type "/Game/AIPhases/Blueprints/Weapon/Data/PDA_Weapon Object Reference")))

(fn `UserConstructionScript`)