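; BP_GM_Loadout is the game mode Blueprint for the Loadout mode in the AIPhases project.
; On BeginPlay it prints an optional debug message, then on authority copies MaxTeamSize from BP_GI_AIPhases, casting and caching the game instance if the reference is not yet valid.
; Tick and the construction script are empty.
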(event `self.ReceiveBeginPlay`
  (`|ExecutionSequence`
    (:`then_0`
      (`self.bShowDebug`
        (:`then`
          (`KismetSystemLibrary.PrintString` "BP_GM_Loadout - EVENT Begin Play" true true (struct :`G` 0.66 :`B` 1.0 :`A` 1.0) 3.0))
        (:`else`)))
    (:`then_1`
      (`/Engine/EditorBlueprintResources/ActorMacros.Switch Has Authority`
        (:`Authority`
          (`self.As BP GI AIPhases`
            (:`then`
              _)
            (:`else`
              (bind _asbp_gi_aiphases (cast `/Game/AIPhases/BP_GI_AIPhases` (`GameplayStatics.GetGameInstance`)))
              (set `self.As BP GI AIPhases` _asbp_gi_aiphases)))
          (set `self.MaxTeamSize` (`/Game/AIPhases/BP_GI_AIPhases.MaxTeamSize` (`self.As BP GI AIPhases`))))))))

(fn `UserConstructionScript`)