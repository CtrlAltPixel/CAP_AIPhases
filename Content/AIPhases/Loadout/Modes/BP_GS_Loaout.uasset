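; Loadout-phase Game State that tracks players in Blue, Red and Spectator team arrays, sized on authority from the Game Mode's max team size.
; Team requests check only slot index validity (Index-1), then remove the player from all teams and set them at Index.
; Outfit and weapon requests check availability but take no action.
; RepNotifies only print debug text; their HUD updates through the player controller are disconnected.
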(event `self.ReceiveBeginPlay`
  (bind _maxteamsize (`/Game/AIPhases/Loadout/Modes/BP_GM_Loadout.MaxTeamSize` (`self.As BP GM Loadout`)))
  (`|ExecutionSequence`
    (:`then_0`
      (`self.bShowDebug`
        (:`then`
          (`KismetSystemLibrary.PrintString` "BP_GS_Loadout - EVENT Begin Play" true true (struct :`G` 0.66 :`B` 1.0 :`A` 1.0) 3.0))
        (:`else`)))
    (:`then_1`
      (`/Engine/EditorBlueprintResources/ActorMacros.Switch Has Authority`
        (:`Authority`
          (`self.As BP GM Loadout`
            (:`then`
              _)
            (:`else`
              (bind _asbp_gm_loadout (cast `/Game/AIPhases/Loadout/Modes/BP_GM_Loadout` (`GameplayStatics.GetGameMode`)))
              (set `self.As BP GM Loadout` _asbp_gm_loadout)))
          (`KismetArrayLibrary.Array_Resize` (`self.BluePlayers`) _maxteamsize)
          (`KismetArrayLibrary.Array_Resize` (`self.SpectatorPlayers`) _maxteamsize)
          (`KismetArrayLibrary.Array_Resize` (`self.RedPlayers`) _maxteamsize))))))

(event `HandleOutfitRequest`
  (params (Outfit :type "SkeletalMesh Object Reference") (Player :type "PlayerController Object Reference"))
  (`|ExecutionSequence`
    (:`then_0`
      (`self.bShowDebug`
        (:`then`
          (`KismetSystemLibrary.PrintString` "BP_GS_Loadout - EVENT Request Outfit" true true (struct :`G` 0.66 :`B` 1.0 :`A` 1.0) 3.0))
        (:`else`)))
    (:`then_1`
      (if (`KismetArrayLibrary.Array_Contains` (`self.Outfits`) Outfit)
        _))))

(event `HandleWeaponRequest`
  (params (WeaponData :type "/Game/AIPhases/Blueprints/Weapon/Data/PDA_Weapon Object Reference") (Player :type "PlayerController Object Reference"))
  (`|ExecutionSequence`
    (:`then_0`
      (`self.bShowDebug`
        (:`then`
          (`KismetSystemLibrary.PrintString` "BP_HUD_Loadout - EVENT Request Weapon" true true (struct :`G` 0.66 :`B` 1.0 :`A` 1.0) 3.0))
        (:`else`)))
    (:`then_1`
      (if (`KismetArrayLibrary.Array_Contains` (`self.Weapon`) WeaponData)
        _))))

(event `HandleTeamRequest`
  (params (Team :type "/Game/AIPhases/Blueprints/Team/Enum/E_Team Enum" :default "NewEnumerator0") (Index :type Integer) (Player :type "PlayerState Object Reference"))
  (`|ExecutionSequence`
    (:`then_0`
      (`self.bShowDebug`
        (:`then`
          (`KismetSystemLibrary.PrintString` "BP_GS_Loadout - EVENT Request Team" true true (struct :`G` 0.66 :`B` 1.0 :`A` 1.0) 3.0))
        (:`else`)))
    (:`then_1`
      (bind _bisvalid (`self.QueryTeam` Team Index))
      (if _bisvalid
        (`self.RemovePlayerFromTeam` Player)
        (`self.AddPlayerToTeam` Team Index Player)))))

(fn `AddPlayerToTeam`
  (params (Team :type "/Game/AIPhases/Blueprints/Team/Enum/E_Team Enum" :default "NewEnumerator0") (Index :type Integer) (Player :type "PlayerState Object Reference"))
  (`|ExecutionSequence`
    (:`then_0`
      (`self.bShowDebug`
        (:`then`
          (`KismetSystemLibrary.PrintString` "BP_PC_CustomLobby - FUNCTION Add Player To Team" true true (struct :`G` 0.66 :`B` 1.0 :`A` 1.0) 3.0))
        (:`else`)))
    (:`then_1`
      (switch `/Game/AIPhases/Blueprints/Team/Enum/E_Team` Team
        (:`NewEnumerator1`
          (`KismetArrayLibrary.Array_Set` (`self.BluePlayers`) (`local.Index`) (`local.Player`) true))
        (:`NewEnumerator3`
          (`KismetArrayLibrary.Array_Set` (`self.SpectatorPlayers`) (`local.Index`) (`local.Player`) true))
        (:`NewEnumerator4`
          (`KismetArrayLibrary.Array_Set` (`self.RedPlayers`) (`local.Index`) (`local.Player`) true))))))

(fn `OnRep_BluePlayers`
  (`|ExecutionSequence`
    (:`then_0`
      (`self.bShowDebug`
        (:`then`
          (`KismetSystemLibrary.PrintString` "BP_GS_Loadout - REPNOTIFY Blue Players" true true (struct :`G` 0.66 :`B` 1.0 :`A` 1.0) 3.0))
        (:`else`)))))

(fn `OnRep_RedPlayers`
  (`|ExecutionSequence`
    (:`then_0`
      (`self.bShowDebug`
        (:`then`
          (`KismetSystemLibrary.PrintString` "BP_GS_Loadout - REPNOTIFY Red Players" true true (struct :`G` 0.66 :`B` 1.0 :`A` 1.0) 3.0))
        (:`else`)))))

(fn `OnRep_SpectatorPlayers`
  (`|ExecutionSequence`
    (:`then_0`
      (`self.bShowDebug`
        (:`then`
          (`KismetSystemLibrary.PrintString` "BP_GS_Loadout - REPNOTIFY Spectator Players" true true (struct :`G` 0.66 :`B` 1.0 :`A` 1.0) 3.0))
        (:`else`)))))

(fn `QueryTeam`
  (params (Team :type "/Game/AIPhases/Blueprints/Team/Enum/E_Team Enum" :default "NewEnumerator0") (Index :type Integer))
  (returns (bIsValid :type Boolean))
  (bind _returnvalue (- Index 1))
  (`|ExecutionSequence`
    (:`then_0`
      (`self.bShowDebug`
        (:`then`
          (`KismetSystemLibrary.PrintString` "BP_PC_CustomLobby - FUNCTION QueryTeam" true true (struct :`G` 0.66 :`B` 1.0 :`A` 1.0) 3.0))
        (:`else`)))
    (:`then_1`
      (switch `/Game/AIPhases/Blueprints/Team/Enum/E_Team` Team
        (:`NewEnumerator1`
          (return (`KismetArrayLibrary.Array_IsValidIndex` (`self.BluePlayers`) _returnvalue)))
        (:`NewEnumerator3`
          (return (`KismetArrayLibrary.Array_IsValidIndex` (`self.SpectatorPlayers`) _returnvalue)))
        (:`NewEnumerator4`
          (return (`KismetArrayLibrary.Array_IsValidIndex` (`self.RedPlayers`) _returnvalue)))))))

(fn `RemovePlayerFromTeam`
  (params (`Player To Remove` :type "PlayerState Object Reference (by ref)"))
  (`|ExecutionSequence`
    (:`then_0`
      (`self.bShowDebug`
        (:`then`
          (`KismetSystemLibrary.PrintString` "BP_PC_CustomLobby - FUNCTION Remove PlayerFromTeam" true true (struct :`G` 0.66 :`B` 1.0 :`A` 1.0) 3.0))
        (:`else`)))
    (:`then_1`
      (`KismetArrayLibrary.Array_RemoveItem` (`self.BluePlayers`) `Player To Remove`)
      (`KismetArrayLibrary.Array_RemoveItem` (`self.RedPlayers`) `Player To Remove`)
      (`KismetArrayLibrary.Array_RemoveItem` (`self.SpectatorPlayers`) `Player To Remove`))))

(fn `UserConstructionScript`)