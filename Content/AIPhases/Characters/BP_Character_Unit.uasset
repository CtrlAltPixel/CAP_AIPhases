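; Character Blueprint for gameplay units, setting trace-channel collision and the gameplay AI controller class on BeginPlay.
; Units without a command controller bind to the GameState's phase-change event, and the AI planning handler adds a StateTree component to the AI controller in the Planning phase.
; MULTI move and montage events bracket each action with start/end calls, whether it succeeds or not.
; On destruction, it reports the death to the GameMode.
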(event `self.ReceiveBeginPlay`
  (`|ExecutionSequence`
    (:`then_0`
      (if (`self.bShowDebug?`)
        (`KismetSystemLibrary.PrintString` "BP_Character_Unit - EVENT BeginPlay" true true (struct :`G` 0.66 :`B` 1.0 :`A` 1.0) 3.0)))
    (:`then_1`
      (`PrimitiveComponent.SetCollisionResponseToChannel` (`self.CapsuleComponent`) "ECC_GameTraceChannel1" "ECR_Block")
      (set `self.AIControllerClass` "/Game/AIPhases/Characters/AI/BP_AIController_Gameplay.BP_AIController_Gameplay_C")
      (`PrimitiveComponent.SetReceivesDecals` (`self.Mesh`) false))))

(event `self.ReceivePossessed`
  (params (NewController :type "Controller Object Reference"))
  (`|ExecutionSequence`
    (:`then_0`
      (if (`self.bShowDebug?`)
        (`KismetSystemLibrary.PrintString` "BP_Character_Unit - EVENT Possessed" true true (struct :`G` 0.66 :`B` 1.0 :`A` 1.0) 3.0)))))

(event `CustomEvent`
  ;[1 0 0 0.5] Comment
  (`self.CommandController`
    (:`then`)
    (:`else`
      (`self.As BP GS Gameplay`
        (:`then`
          _)
        (:`else`
          (bind _asbp_gs_gameplay (cast `/Game/AIPhases/Modes/BP_GS_Gameplay` (`GameplayStatics.GetGameState`)))
          (set `self.As BP GS Gameplay` _asbp_gs_gameplay)))
      (add `/Game/AIPhases/Modes/BP_GS_Gameplay.OnPhaseChange` (`self.As BP GS Gameplay`) (`|CreateDelegate` :!event `OnAIPlanning`)))))

(event `OnAIPlanning`
  (params (Phase :type "/Game/AIPhases/Modes/Enums/E_Phase Enum" :default "NewEnumerator0"))
  ;[1 0 0 0.5] Comment
  (switch `/Game/AIPhases/Modes/Enums/E_Phase` Phase
    (:`NewEnumerator0`
      (`AddComponent|NODE_AddStateTreeAIComponent-0` :`self` (`AIBlueprintHelperLibrary.GetAIController` self)))))

(event `MULTIMoveTo`
  (params (Destination :type "Vector Structure"))
  (`|AIMoveTo` self Destination null
    (:`then`
      (`self.OnActionStart`))
    (:`OnSuccess`
      (`self.OnActionEnd` :!label _label))
    (:`OnFail`
      (goto _label))))

(event `MULTIPlayMontage`
  (params (AnimMontage :type "AnimMontage Object Reference"))
  (bind _output_get (set `self.AsCurrentAnimMontage` AnimMontage))
  (`|PlayMontage` (`self.Mesh`) _output_get
    (:`then`
      (`self.OnActionStart`))
    (:`OnCompleted`
      (set `self.AsCurrentAnimMontage` null :!label _label_2)
      (`self.OnActionEnd`))
    (:`OnBlendOut`
      (goto _label_2))
    (:`OnInterrupted`
      (goto _label_2))))

(event `self.ReceiveDestroyed`
  (bind _as_bp_gm_aiphases (`self.As BP GM AIPhases`)
    (:`then`
      _)
    (:`else`
      (bind _asbp_gm_gameplay (cast `/Game/AIPhases/Modes/BP_GM_Gameplay` (`GameplayStatics.GetGameMode`)))
      (set `self.As BP GM AIPhases` _asbp_gm_gameplay)))
  (`/Game/AIPhases/Modes/BP_GM_Gameplay.OnCharacterDied` _as_bp_gm_aiphases self))

(fn `UserConstructionScript`)