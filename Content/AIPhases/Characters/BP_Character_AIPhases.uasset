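; Character for the AIPhases mode, with hover and selection feedback and AI controller class assignment.
; BeginPlay caches game mode and HUD, configures collision and a capsule-scaled decal, and creates dynamic decal and outline materials.
; Cursor hover toggles the mesh's outline overlay, while interact events toggle the decal and update the HUD's selected-character window.
; A multicast montage event raises start/end callbacks, and destruction reports the character's death to the game mode.
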(event `self.ReceiveBeginPlay`
  (`self.InitCasts`)
  (`self.InitCharacter`)
  (`self.InitMaterialDecalInteract`)
  (`self.InitMaterialOverlayOutline`))

(event `self.ReceiveActorBeginCursorOver`
  (`MeshComponent.SetOverlayMaterial` (`self.Mesh`) (`self.AsMatOverlayOutline`)))

(event `self.ReceiveActorEndCursorOver`
  (`MeshComponent.SetOverlayMaterial` (`self.Mesh`) null))

(event `EventActorBeginInteract`
  (`SceneComponent.SetVisibility` (`self.Decal_interact`) true false)
  (bind _aslocalplayerhud (`self.AsLocalPlayerHUD`)
    (:`then`
      (`/Game/AIPhases/UI/HUD/BP_HUD_AIPhases.UpdateSelectedCharacterWindow` _aslocalplayerhud self))
    (:`else`)))

(event `EventActorEndInteract`
  (`SceneComponent.SetVisibility` (`self.Decal_interact`) false false)
  (bind _aslocalplayerhud (`self.AsLocalPlayerHUD`)
    (:`then`
      (`/Game/AIPhases/UI/HUD/BP_HUD_AIPhases.UpdateSelectedCharacterWindow` _aslocalplayerhud null))
    (:`else`)))

(event `MULTIPlayMontage`
  (params (AnimMontage :type "AnimMontage Object Reference"))
  (bind _output_get (set `self.AsCurrentAnimMontage` AnimMontage))
  (`|PlayMontage` (`self.Mesh`) _output_get
    (:`then`
      (`self.OnMontageStart`))
    (:`OnCompleted`
      (set `self.AsCurrentAnimMontage` null)
      (`self.OnMontageEnd`))))

(event `self.ReceiveDestroyed`
  (bind _as_bp_gm_aiphases (`self.As BP GM AIPhases`)
    (:`then`
      (`/Game/AIPhases/Modes/BP_GM_AIPhases.OnCharacterDied` _as_bp_gm_aiphases self))
    (:`else`)))

(fn `InitCasts`
  (bind _asbp_gm_aiphases (cast `/Game/AIPhases/Modes/BP_GM_AIPhases` (`GameplayStatics.GetGameMode`)))
  (set `self.As BP GM AIPhases` _asbp_gm_aiphases)
  (bind _asbp_hud_aiphases (cast `/Game/AIPhases/UI/HUD/BP_HUD_AIPhases` (`PlayerController.GetHUD` (`GameplayStatics.GetPlayerController` 0))))
  (set `self.AsLocalPlayerHUD` _asbp_hud_aiphases))

(fn `InitCharacter`
  (bind _capsulecomponent (`self.CapsuleComponent`))
  (bind _returnvalue (/ (`CapsuleComponent.CapsuleRadius` _capsulecomponent) 100.0))
  (`PrimitiveComponent.SetCollisionResponseToChannel` (`self.CapsuleComponent`) "ECC_GameTraceChannel1" "ECR_Block")
  (`SceneComponent.SetRelativeScale3D` (`self.Decal_interact`) (`KismetMathLibrary.MakeVector` (/ (`CapsuleComponent.CapsuleHalfHeight` _capsulecomponent) 100.0) _returnvalue _returnvalue))
  (`SceneComponent.SetVisibility` (`self.Decal_interact`) false false)
  (`PrimitiveComponent.SetReceivesDecals` (`self.Mesh`) false)
  (set `self.AIControllerClass` "/Game/AIPhases/Characters/AI/BP_AIController_AIPhases.BP_AIController_AIPhases_C"))

(fn `InitMaterialDecalInteract`
  (bind _returnvalue (`KismetMaterialLibrary.CreateDynamicMaterialInstance` "/Game/AIPhases/Characters/Material/MAT_Decal_Selected.MAT_Decal_Selected"))
  (bind _output_get (set `self.AsMATDecalInteract` _returnvalue))
  (`MaterialInstanceDynamic.SetVectorParameterValue` _output_get "Color" (struct :`R` 1.0 :`G` 1.0 :`B` 1.0 :`A` 1.0))
  (`DecalComponent.SetDecalMaterial` (`self.Decal_interact`) (`self.AsMATDecalInteract`)))

(fn `InitMaterialOverlayOutline`
  (bind _returnvalue (`KismetMaterialLibrary.CreateDynamicMaterialInstance` "/Game/AIPhases/Characters/Material/MAT_Overlay_Outline.MAT_Overlay_Outline"))
  (bind _output_get (set `self.AsMatOverlayOutline` _returnvalue))
  (`MaterialInstanceDynamic.SetVectorParameterValue` _output_get "Color" (struct :`G` 1.0 :`B` 1.0 :`A` 1.0)))

(fn `UserConstructionScript`)