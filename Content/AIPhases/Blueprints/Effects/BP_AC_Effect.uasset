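; Actor component for a turn-limited gameplay effect that expires after a duration taken from its EffectData.
; BeginPlay computes an expiry turn from the turn count and binds to the gameplay GameState's turn-change event.
; Turn updates broadcast OnEffectStart until the expiry turn, when the component broadcasts OnEffectEnd and destroys itself.
; The phase-change handler only prints debug text, and its binding is unconnected.
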(event `self.ReceiveBeginPlay`
  (`|ExecutionSequence`
    (:`then_0`
      (`self.bShowDebug?`
        (:`then`
          (`KismetSystemLibrary.PrintString` "BP_AC_Effect - EVENT Begin Play" true true (struct :`G` 0.66 :`B` 1.0 :`A` 1.0) 3.0))
        (:`else`)))
    (:`then_1`
      (bind _effectdata (`self.EffectData`)
        (:`then`
          (set `self.LifeTime` (+ (`/Game/AIPhases/Gameplay/Modes/BP_GS_Gameplay.TurnCount` (`self.As BP GS Gameplay`)) (`/Game/AIPhases/Blueprints/Effects/Data/PDA_Effect.TurnCount` _effectdata))))
        (:`else`)))
    (:`then_2`
      (`self.As BP GS Gameplay`
        (:`then`
          _)
        (:`else`
          (bind _asbp_gs_gameplay (cast `/Game/AIPhases/Gameplay/Modes/BP_GS_Gameplay` (`GameplayStatics.GetGameState`)))
          (set `self.As BP GS Gameplay` _asbp_gs_gameplay)))
      (add `/Game/AIPhases/Gameplay/Modes/BP_GS_Gameplay.OnTurnChange` (`self.As BP GS Gameplay`) (`|CreateDelegate` :!event `HandleTurnUpdate`)))))

(event `HandleTurnUpdate`
  (params (TurnCount :type Integer))
  (`|ExecutionSequence`
    (:`then_0`
      (`self.bShowDebug?`
        (:`then`
          (`KismetSystemLibrary.PrintString` "BP_AC_Effect - EVENT Handle Turn Update" true true (struct :`G` 0.66 :`B` 1.0 :`A` 1.0) 3.0))
        (:`else`)))
    (:`then_1`
      (if (== TurnCount (`self.LifeTime`))
        (`self.EffectEnd`)
        (else
          (`self.EffectStart`))))))

(event `EffectStart`
  (`|ExecutionSequence`
    (:`then_0`
      (`self.bShowDebug?`
        (:`then`
          (`KismetSystemLibrary.PrintString` "BP_AC_Effect - EVENT Effect Activate" true true (struct :`G` 0.66 :`B` 1.0 :`A` 1.0) 3.0))
        (:`else`)))
    (:`then_1`
      (`self.OnEffectStart` self))))

(event `EffectEnd`
  (`|ExecutionSequence`
    (:`then_0`
      (`self.bShowDebug?`
        (:`then`
          (`KismetSystemLibrary.PrintString` "BP_AC_Effect - EVENT Effect Activate" true true (struct :`G` 0.66 :`B` 1.0 :`A` 1.0) 3.0))
        (:`else`)))
    (:`then_1`
      (`self.OnEffectEnd` self))
    (:`then_2`
      (`self.K2_DestroyComponent`))))

(event `HandlePhaseUpdate`
  (params (Phase :type "/Game/AIPhases/Blueprints/Turns/Enums/E_Phase Enum" :default "NewEnumerator6"))
  (`|ExecutionSequence`
    (:`then_0`
      (`self.bShowDebug?`
        (:`then`
          (`KismetSystemLibrary.PrintString` "BP_AC_Effect - EVENT Handle Phase Update" true true (struct :`G` 0.66 :`B` 1.0 :`A` 1.0) 3.0))
        (:`else`)))))