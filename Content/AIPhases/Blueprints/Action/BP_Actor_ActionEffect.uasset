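; BP_Actor_ActionEffect is an actor in the AIPhases action system that signals when an action effect starts and ends.
; Its Action Start and Action End events each fire a matching event dispatcher, OnActionEffectStart or OnActionEffectEnd.
; BeginPlay and both events can print debug messages behind the ShowDebug flag.
; It contains no effect logic of its own.
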(event `self.ReceiveBeginPlay`
  (`|ExecutionSequence`
    (:`then_0`
      (if (`self.bShowDebug?`)
        (`KismetSystemLibrary.PrintString` "BP_Actor_ActionEffect - EVENT Begin Play" true true (struct :`G` 0.66 :`B` 1.0 :`A` 1.0) 3.0)))))

(event `EventActionStart`
  (`|ExecutionSequence`
    (:`then_0`
      (if (`self.bShowDebug?`)
        (`KismetSystemLibrary.PrintString` "BP_Actor_ActionEffect - EVENT Action Start" true true (struct :`G` 0.66 :`B` 1.0 :`A` 1.0) 3.0)))
    (:`then_1`
      (`self.OnActionEffectStart`))))

(event `EventActionEnd`
  (`|ExecutionSequence`
    (:`then_0`
      (if (`self.bShowDebug?`)
        (`KismetSystemLibrary.PrintString` "BP_Actor_ActionEffect - EVENT Action End" true true (struct :`G` 0.66 :`B` 1.0 :`A` 1.0) 3.0)))
    (:`then_1`
      (`self.OnActionEffectEnd`))))

(fn `UserConstructionScript`)