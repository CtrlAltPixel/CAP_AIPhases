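; BP_Actor_Action is an actor that represents one AI action performed by a Caster, configured through ActionData.
; On BeginPlay it plays the ActionData montage through the Caster's BP_AIController_Gameplay.
; ActionStart and ActionEnd events broadcast the OnActionStart and OnActionEnd dispatchers, with optional debug prints.
; A disconnected loop would add each ActionData effect as a component on every target, so no effects are applied here.
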(event `self.ReceiveBeginPlay`
  (`|ExecutionSequence`
    (:`then_0`
      (`self.bShowDebug?`
        (:`then`
          (`KismetSystemLibrary.PrintString` "BP_Actor_ActionEffect - EVENT Begin Play" true true (struct :`G` 0.66 :`B` 1.0 :`A` 1.0) 3.0))
        (:`else`)))
    (:`then_1`
      (bind _actiondata (`self.ActionData`)
        (:`then`)
        (:`else`)))
    (:`then_2`
      (bind _actiondata_2 (`self.ActionData`)
        (:`then`
          (bind _caster (`self.Caster`)
            (:`then`
              (bind _asbp_aicontroller_gameplay (cast `/Game/AIPhases/Blueprints/Units/AI/BP_AIController_Gameplay` (`AIBlueprintHelperLibrary.GetAIController` _caster)))
              (`/Game/AIPhases/Blueprints/Units/AI/BP_AIController_Gameplay.PlayMontage` _asbp_aicontroller_gameplay (`/Game/AIPhases/Blueprints/Action/Data/PDA_Action.Montage` _actiondata_2)))
            (:`else`)))
        (:`else`)))))

(event `ActionStart`
  (`|ExecutionSequence`
    (:`then_0`
      (`self.bShowDebug?`
        (:`then`
          (`KismetSystemLibrary.PrintString` "BP_Actor_ActionEffect - EVENT Action Start" true true (struct :`G` 0.66 :`B` 1.0 :`A` 1.0) 3.0))
        (:`else`)))
    (:`then_1`
      (`self.OnActionStart` self))))

(event `ActionEnd`
  (`|ExecutionSequence`
    (:`then_0`
      (`self.bShowDebug?`
        (:`then`
          (`KismetSystemLibrary.PrintString` "BP_Actor_ActionEffect - EVENT Action End" true true (struct :`G` 0.66 :`B` 1.0 :`A` 1.0) 3.0))
        (:`else`)))
    (:`then_1`
      (`self.OnActionEnd` self))))

(fn `UserConstructionScript`)