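; BP_Actor_Target is a target actor in the AIPhases Targets folder, currently a skeleton with no gameplay behavior.
; BeginPlay, Tick, TargetStart and TargetEnd each print a debug message gated by a validity check on ShowDebug.
; Tick also checks TargetData and switches on its Shape, but the switch has no branch logic yet.
; The construction script is empty and the overlap event is disabled.
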(event `self.ReceiveTick`
  (params (DeltaSeconds :type "Float (single-precision)"))
  (`|ExecutionSequence`
    (:`then_0`
      (`self.bShowDebug`
        (:`then`
          (`KismetSystemLibrary.PrintString` "BP_Actor_Target - EVENT Tick" true true (struct :`G` 0.66 :`B` 1.0 :`A` 1.0) 3.0))
        (:`else`)))
    (:`then_1`
      (bind _targetdata (`self.TargetData`)
        (:`then`
          (switch `/Game/AIPhases/E_Shape` (`/Game/AIPhases/Blueprints/Targets/Data/PDA_Target.Shape` _targetdata)))
        (:`else`)))))

(event `self.ReceiveBeginPlay`
  (`|ExecutionSequence`
    (:`then_0`
      (`self.bShowDebug`
        (:`then`
          (`KismetSystemLibrary.PrintString` "BP_Actor_Target - EVENT Begin Play" true true (struct :`G` 0.66 :`B` 1.0 :`A` 1.0) 3.0))
        (:`else`)))))

(event `Target Start`
  (`|ExecutionSequence`
    (:`then_0`
      (`self.bShowDebug`
        (:`then`
          (`KismetSystemLibrary.PrintString` "BP_Actor_Target - EVENT Target Start" true true (struct :`G` 0.66 :`B` 1.0 :`A` 1.0) 3.0))
        (:`else`)))))

(event `Target End`
  (`|ExecutionSequence`
    (:`then_0`
      (`self.bShowDebug`
        (:`then`
          (`KismetSystemLibrary.PrintString` "BP_Actor_Target - EVENT Target End" true true (struct :`G` 0.66 :`B` 1.0 :`A` 1.0) 3.0))
        (:`else`)))))

(fn `UserConstructionScript`)