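; BP_AC_Interact is an interaction Blueprint in the AIPhases content, currently a skeleton with no gameplay logic.
; It exposes InteractStart and InteractEnd events alongside BeginPlay.
; Each event only prints a debug string naming itself, gated by a validity check on ShowDebug.
; Tick is disabled.
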(event `self.ReceiveBeginPlay`
  (`|ExecutionSequence`
    (:`then_0`
      (`self.bShowDebug`
        (:`then`
          (`KismetSystemLibrary.PrintString` "BP_AC_Interact - EVENT Begin Play" true true (struct :`G` 0.66 :`B` 1.0 :`A` 1.0) 3.0))
        (:`else`)))))

(event `/Game/AIPhases/Blueprints/Interact/Interface/BPI_Interact.InteractStart`
  (`|ExecutionSequence`
    (:`then_0`
      (`self.bShowDebug`
        (:`then`
          (`KismetSystemLibrary.PrintString` "BP_AC_Interact - EVENT InteractStart" true true (struct :`G` 0.66 :`B` 1.0 :`A` 1.0) 3.0))
        (:`else`)))))

(event `/Game/AIPhases/Blueprints/Interact/Interface/BPI_Interact.InteractEnd`
  (`|ExecutionSequence`
    (:`then_0`
      (`self.bShowDebug`
        (:`then`
          (`KismetSystemLibrary.PrintString` "BP_AC_Interact - EVENT Interact End" true true (struct :`G` 0.66 :`B` 1.0 :`A` 1.0) 3.0))
        (:`else`)))))