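; BP_AC_Attributes is an attribute component that holds a keyed map of attribute structs, with lookup and update functions.
; UpdateAttribute checks that the name exists, then branches to Base, Bonus or Current handlers, passing Current a zero instead of its Value input.
; Base and Bonus are debug-print stubs.
; Current adds its value to the struct and fires OnUpdateAttribute, with no explicit write back to the map.
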(fn `GetAttribute`
  (params (Key :type Name))
  (returns (Value :type "/Game/AIPhases/Blueprints/Attributes/S_Attribute Structure") (ReturnValue :type Boolean))
  (bind (_value _returnvalue) (`BlueprintMapLibrary.Map_Find` (`self.Attributes`) Key))
  (`|ExecutionSequence`
    (:`then_0`
      (`self.bShowDebug?`
        (:`then`
          (`KismetSystemLibrary.PrintString` "BP_AC_Attribute - FUNCTION Get Attribute" true true (struct :`G` 0.66 :`B` 1.0 :`A` 1.0) 3.0))
        (:`else`)))
    (:`then_1`
      (return _value _returnvalue))))

(fn `UpdateAttribute`
  (params (Name :type Name) (Value :type "Float (double-precision)") (Attribute :type "/Game/AIPhases/Blueprints/Attributes/E_Attribute Enum" :default "NewEnumerator0"))
  (`|ExecutionSequence`
    (:`then_0`
      (`self.bShowDebug?`
        (:`then`
          (`KismetSystemLibrary.PrintString` "BP_AC_Attribute - FUNCTION Update Attribute" true true (struct :`G` 0.66 :`B` 1.0 :`A` 1.0) 3.0))
        (:`else`)))
    (:`then_1`
      (bind (_value _returnvalue) (`self.GetAttribute` Name))
      (if _returnvalue
        (switch `/Game/AIPhases/Blueprints/Attributes/E_Attribute` (`local.Attribute`)
          (:`NewEnumerator1`
            (`self.UpdateAttributeBase`))
          (:`NewEnumerator2`
            (`self.UpdateAttributeBonus`))
          (:`NewEnumerator3`
            (`self.UpdateAttributeCurrent` (struct))))))))

(fn `UpdateAttributeBase`
  (`|ExecutionSequence`
    (:`then_0`
      (`self.bShowDebug?`
        (:`then`
          (`KismetSystemLibrary.PrintString` "BP_AC_Attribute - FUNCTION Update Attribute Base" true true (struct :`G` 0.66 :`B` 1.0 :`A` 1.0) 3.0))
        (:`else`)))))

(fn `UpdateAttributeBonus`
  (`|ExecutionSequence`
    (:`then_0`
      (`self.bShowDebug?`
        (:`then`
          (`KismetSystemLibrary.PrintString` "BP_AC_Attribute - FUNCTION Update AttributeBonus" true true (struct :`G` 0.66 :`B` 1.0 :`A` 1.0) 3.0))
        (:`else`)))))

(fn `UpdateAttributeCurrent`
  (params (Attribute :type "/Game/AIPhases/Blueprints/Attributes/S_Attribute Structure") (Value :type "Float (double-precision)"))
  (`|ExecutionSequence`
    (:`then_0`
      (`self.bShowDebug?`
        (:`then`
          (`KismetSystemLibrary.PrintString` "BP_AC_Attribute - FUNCTION Update Attribute Current" true true (struct :`G` 0.66 :`B` 1.0 :`A` 1.0) 3.0))
        (:`else`)))
    (:`then_1`
      (bind _structout (setmembers `/Game/AIPhases/Blueprints/Attributes/S_Attribute` :`StructRef` (`local.Attribute`) :`Current` (+ (`.Current_12_353020DF4030D8E88DC1DD9CD47A9DB3` (break `/Game/AIPhases/Blueprints/Attributes/S_Attribute` (`local.Attribute`))) Value)))
      (`self.OnUpdateAttribute` _structout))))