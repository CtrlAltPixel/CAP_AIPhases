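; BP_AC_Team is a team component, apparently an actor component in the AIPhases content, that stores its owner's Team value.
; GetTeam returns the stored value and SetTeam overwrites it, with no other team logic in the graphs.
; BeginPlay and both functions print debug messages gated by an IsValid check on ShowDebug, though SetTeam's message is mislabeled as Get Team.
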(event `self.ReceiveBeginPlay`
  (`|ExecutionSequence`
    (:`then_0`
      (`self.bShowDebug?`
        (:`then`
          (`KismetSystemLibrary.PrintString` "BP_AC_Team - EVENT Begin Play" true true (struct :`G` 0.66 :`B` 1.0 :`A` 1.0) 3.0))
        (:`else`)))
    (:`then_1`)))

(fn `GetTeam`
  (returns (Team :type "/Game/AIPhases/Blueprints/Team/Enum/E_Team Enum"))
  (`|ExecutionSequence`
    (:`then_0`
      (`self.bShowDebug?`
        (:`then`
          (`KismetSystemLibrary.PrintString` "BP_AC_Team - FUNCTION Get Team" true true (struct :`G` 0.66 :`B` 1.0 :`A` 1.0) 3.0))
        (:`else`)))
    (:`then_1`
      (return (`self.Team`)))))

(fn `SetTeam`
  (params (Team :type "/Game/AIPhases/Blueprints/Team/Enum/E_Team Enum" :default "NewEnumerator0"))
  (`|ExecutionSequence`
    (:`then_0`
      (`self.bShowDebug?`
        (:`then`
          (`KismetSystemLibrary.PrintString` "BP_AC_Team - FUNCTION Get Team" true true (struct :`G` 0.66 :`B` 1.0 :`A` 1.0) 3.0))
        (:`else`)))
    (:`then_1`
      (set `self.Team` Team))))