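; BP_AC_Weapon is a weapon component in the AIPhases content that holds weapon data for its owner.
; SetWeapon stores the incoming WeaponData, while GetWeapon shows only a debug print and no retrieval logic.
; BeginPlay and both functions print trace messages when ShowDebug is valid, though SetWeapon's message is mislabelled as Get Weapon.
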(event `self.ReceiveBeginPlay`
  (`|ExecutionSequence`
    (:`then_0`
      (`self.bShowDebug`
        (:`then`
          (`KismetSystemLibrary.PrintString` "BP_AC_Weapon - EVENT Begin Play" true true (struct :`G` 0.66 :`B` 1.0 :`A` 1.0) 3.0))
        (:`else`)))))

(fn `GetWeapon`
  (`|ExecutionSequence`
    (:`then_0`
      (`self.bShowDebug`
        (:`then`
          (`KismetSystemLibrary.PrintString` "BP_AC_Weapon - FUNCTION Get Weapon" true true (struct :`G` 0.66 :`B` 1.0 :`A` 1.0) 3.0))
        (:`else`)))))

(fn `SetWeapon`
  (params (WeaponData :type "/Game/AIPhases/Blueprints/Weapon/Data/PDA_Weapon Object Reference"))
  (`|ExecutionSequence`
    (:`then_0`
      (`self.bShowDebug`
        (:`then`
          (`KismetSystemLibrary.PrintString` "BP_AC_Weapon - FUNCTION Get Weapon" true true (struct :`G` 0.66 :`B` 1.0 :`A` 1.0) 3.0))
        (:`else`)))
    (:`then_1`
      (set `self.WeaponData` WeaponData))))