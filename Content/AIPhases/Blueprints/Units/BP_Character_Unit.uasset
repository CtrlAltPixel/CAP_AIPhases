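; BP_Character_Unit is a player-commanded unit character, driven by the gameplay AI controller class set on BeginPlay.
; Setting its CommandPlayerState registers the unit with that BP_PS_Gameplay and copies over team, outfit and weapon data.
; RepNotifies apply those values to the team decal color, skeletal mesh and main/off-hand weapon meshes.
; Multi-prefixed events handle AI movement, relocation and montage playback.
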(event `self.ReceiveBeginPlay`
  (`|ExecutionSequence`
    (:`then_0`
      (`self.bShowDebug?`
        (:`then`
          (`KismetSystemLibrary.PrintString` "BP_Character_Unit - EVENT BeginPlay" true true (struct :`G` 0.66 :`B` 1.0 :`A` 1.0) 3.0))
        (:`else`)))
    (:`then_1`
      (`PrimitiveComponent.SetCollisionResponseToChannel` (`self.CapsuleComponent`) "ECC_GameTraceChannel1" "ECR_Block")
      (set `self.AIControllerClass` "/Game/AIPhases/Blueprints/Units/AI/BP_AIController_Gameplay.BP_AIController_Gameplay_C")
      (`PrimitiveComponent.SetReceivesDecals` (`self.Mesh`) false))))

(event `UpdateCommandPlayerState`
  (params (CommandPlayerState :type "/Game/AIPhases/Gameplay/Player/BP_PS_Gameplay Object Reference"))
  (`|ExecutionSequence`
    (:`then_0`
      (`self.bShowDebug?`
        (:`then`
          (`KismetSystemLibrary.PrintString` "BP_Character_Unit - EVENT Update Command Player State" true true (struct :`G` 0.66 :`B` 1.0 :`A` 1.0) 3.0))
        (:`else`)))
    (:`then_1`
      (set `self.CommandPlayerState` CommandPlayerState))))

(event `MULTIPlayMontage`
  (params (MontageToPlay :type "AnimMontage Object Reference"))
  (`|ExecutionSequence`
    (:`then_0`
      (`self.bShowDebug?`
        (:`then`
          (`KismetSystemLibrary.PrintString` "BP_Character_Unit - EVENT Update Command Player State" true true (struct :`G` 0.66 :`B` 1.0 :`A` 1.0) 3.0))
        (:`else`)))
    (:`then_1`
      (`|PlayMontage` (`self.Mesh`) MontageToPlay))))

(event `UpdateTeam`
  (params (Team :type "/Game/AIPhases/Blueprints/Team/Enum/E_Team Enum" :default "NewEnumerator0"))
  (`|ExecutionSequence`
    (:`then_0`
      (`self.bShowDebug?`
        (:`then`
          (`KismetSystemLibrary.PrintString` "BP_Character_Unit - EVENT Update Team" true true (struct :`G` 0.66 :`B` 1.0 :`A` 1.0) 3.0))
        (:`else`)))
    (:`then_1`
      (set `self.Team` Team))))

(event `MultiMoveTo`
  (params (Location :type "Vector Structure"))
  (`|ExecutionSequence`
    (:`then_0`
      (`self.bShowDebug?`
        (:`then`
          (`KismetSystemLibrary.PrintString` "BP_Character_Unit - EVENT Move to" true true (struct :`G` 0.66 :`B` 1.0 :`A` 1.0) 3.0))
        (:`else`)))
    (:`then_1`
      (`|AIMoveTo` null Location null))))

(event `UpdateOutfit`
  (params (Outfit :type "SkeletalMesh Object Reference"))
  (`|ExecutionSequence`
    (:`then_0`
      (if (`self.bShowDebug?`)
        (`KismetSystemLibrary.PrintString` "BP_Character_Unit - EVENT UpdateMesh" true true (struct :`G` 0.66 :`B` 1.0 :`A` 1.0) 3.0)))
    (:`then_1`
      (set `self.Outfit` Outfit))))

(event `MULTISetActorLocation`
  (params (Location :type "Vector Structure"))
  (`|ExecutionSequence`
    (:`then_0`
      (`self.bShowDebug?`
        (:`then`
          (`KismetSystemLibrary.PrintString` "BP_Character_Unit - EVENT Set Location" true true (struct :`G` 0.66 :`B` 1.0 :`A` 1.0) 3.0))
        (:`else`)))
    (:`then_1`
      (`self.K2_SetActorLocation` Location))))

(event `UpdateWeapon`
  (params (WeaponData :type "/Game/AIPhases/Blueprints/Weapon/Data/PDA_Weapon Object Reference"))
  (`|ExecutionSequence`
    (:`then_0`
      (if (`self.bShowDebug?`)
        (`KismetSystemLibrary.PrintString` "BP_Character_Unit - EVENT Update Weapon Data" true true (struct :`G` 0.66 :`B` 1.0 :`A` 1.0) 3.0)))
    (:`then_1`
      (set `self.WeaponData` WeaponData))))

(fn `OnRep_CommandPlayerState`
  (`|ExecutionSequence`
    (:`then_0`
      (`self.bShowDebug?`
        (:`then`
          (`KismetSystemLibrary.PrintString` "BP_Character_Unit - REPNOTIFY Update Unit" true true (struct :`G` 0.66 :`B` 1.0 :`A` 1.0) 3.0))
        (:`else`)))
    (:`then_1`
      (bind _commandplayerstate (`self.CommandPlayerState`)
        (:`then`
          (bind _asbp_ps_gameplay (cast `/Game/AIPhases/Gameplay/Player/BP_PS_Gameplay` _commandplayerstate))
          (`/Game/AIPhases/Gameplay/Player/BP_PS_Gameplay.UpdateUnit` _asbp_ps_gameplay self)
          (`self.UpdateTeam` (`/Game/AIPhases/Gameplay/Player/BP_PS_Gameplay.Team` _asbp_ps_gameplay))
          (`self.UpdateOutfit` (`/Game/AIPhases/Gameplay/Player/BP_PS_Gameplay.Outfit` _asbp_ps_gameplay))
          (`self.UpdateWeapon` (`/Game/AIPhases/Gameplay/Player/BP_PS_Gameplay.WeaponData` _asbp_ps_gameplay)))
        (:`else`)))))

(fn `OnRep_Outfit`
  (`|ExecutionSequence`
    (:`then_0`
      (if (`self.bShowDebug?`)
        (`KismetSystemLibrary.PrintString` "BP_Character_Unit - REPNOTIFY Outfit" true true (struct :`G` 0.66 :`B` 1.0 :`A` 1.0) 3.0)))
    (:`then_1`
      (`SkeletalMeshComponent.SetSkeletalMeshAsset` (`self.Mesh`) (`self.Outfit`)))))

(fn `OnRep_Team`
  (`|ExecutionSequence`
    (:`then_0`
      (`self.bShowDebug?`
        (:`then`
          (`KismetSystemLibrary.PrintString` "BP_Character_Unit - REPNOTIFY Team" true true (struct :`G` 0.66 :`B` 1.0 :`A` 1.0) 3.0))
        (:`else`)))
    (:`then_1`
      (`DecalComponent.SetDecalColor` (`self.Decal_Team`) (select `/Game/AIPhases/Blueprints/Team/Enum/E_Team` (`self.Team`) :!type "LinearColor Structure")))))

(fn `OnRep_WeaponData`
  (`|ExecutionSequence`
    (:`then_0`
      (if (`self.bShowDebug?`)
        (`KismetSystemLibrary.PrintString` "BP_Character_Unit - REPNOTIFY Weapon data" true true (struct :`G` 0.66 :`B` 1.0 :`A` 1.0) 3.0)))
    (:`then_1`
      (bind _weapondata (`self.WeaponData`)
        (:`then`
          (`StaticMeshComponent.SetStaticMesh` (`self.BP_SMC_Weapon_MainHand`) (`/Game/AIPhases/Blueprints/Weapon/Data/PDA_Weapon.MeshMainHand` _weapondata))
          (`StaticMeshComponent.SetStaticMesh` (`self.BP_SMC_Weapon_OffHand`) (`/Game/AIPhases/Blueprints/Weapon/Data/PDA_Weapon.MeshOffHand` _weapondata)))
        (:`else`)))))

(fn `UserConstructionScript`
  (`|ExecutionSequence`
    (:`then_0`
      (if (`self.bShowDebug?`)
        (`KismetSystemLibrary.PrintString` "BP_Character_Unit - EVENT BeginPlay" true true (struct :`G` 0.66 :`B` 1.0 :`A` 1.0) 3.0)))))