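; AI controller for gameplay units in a phase-based game, driving non-player turns through a melee StateTree.
; AITurnStart sends StateTree events tagged for Planning, Movement or Combat, while per-phase update events store action data.
; PlayMontage and MoveTo forward to the controlled BP_Character_Unit's multicast functions.
; Bots bind to the game state's phase change, but HandlePhaseChange only disables StateTree auto-start; StartLogic calls, including the ranged tree's, are unwired.
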(event `self.ReceiveBeginPlay`
  (`|ExecutionSequence`
    (:`then_0`
      (`self.bShowDebug?`
        (:`then`
          (`KismetSystemLibrary.PrintString` "BP_Character_Unit - EVENT Begin Play" true true (struct :`G` 0.66 :`B` 1.0 :`A` 1.0) 3.0))
        (:`else`)))
    (:`then_1`
      (switch `/Game/AIPhases/Blueprints/Units/Enum/E_Commander` (`self.Command`)
        (:`NewEnumerator1`
          (`self.As BP GS Gameplay`
            (:`then`
              _)
            (:`else`
              (bind _asbp_gs_gameplay (cast `/Game/AIPhases/Gameplay/Modes/BP_GS_Gameplay` (`GameplayStatics.GetGameState`)))
              (set `self.As BP GS Gameplay` _asbp_gs_gameplay)))
          (add `/Game/AIPhases/Gameplay/Modes/BP_GS_Gameplay.OnPhaseChange` (`self.As BP GS Gameplay`) (`|CreateDelegate` :!event `HandlePhaseChange`)))))))

(event `self.ReceivePossess`
  (params (PossessedPawn :type "Pawn Object Reference"))
  (`|ExecutionSequence`
    (:`then_0`
      (`self.bShowDebug?`
        (:`then`
          (`KismetSystemLibrary.PrintString` "BP_Character_Unit - EVENT On Possess" true true (struct :`G` 0.66 :`B` 1.0 :`A` 1.0) 3.0))
        (:`else`)))
    (:`then_1`
      (bind _asbp_character_unit (cast `/Game/AIPhases/Blueprints/Units/BP_Character_Unit` PossessedPawn))
      (set `self.Command Player State` (`/Game/AIPhases/Blueprints/Units/BP_Character_Unit.CommandPlayerState` _asbp_character_unit)))))

(event `SpellActionUpdate`
  (params (ActionData :type "/Game/AIPhases/Blueprints/Action/Data/PDA_Action Object Reference"))
  (`|ExecutionSequence`
    (:`then_0`
      (`self.bShowDebug?`
        (:`then`
          (`KismetSystemLibrary.PrintString` "BP_Character_Unit - EVENT Spell Action Update" true true (struct :`G` 0.66 :`B` 1.0 :`A` 1.0) 3.0))
        (:`else`)))
    (:`then_1`
      (set `self.SpellActionData` ActionData))))

(event `HandlePhaseChange`
  (params (Phase :type "/Game/AIPhases/Blueprints/Turns/Enums/E_Phase Enum" :default "NewEnumerator6"))
  (`|ExecutionSequence`
    (:`then_0`
      (`self.bShowDebug?`
        (:`then`
          (`KismetSystemLibrary.PrintString` "BP_Character_Unit - EVENT Handle Phase Change" true true (struct :`G` 0.66 :`B` 1.0 :`A` 1.0) 3.0))
        (:`else`)))
    (:`then_1`
      (`StateTreeComponent.SetStartLogicAutomatically` (`self.StateTreeAI_Melee`) false)
      (switch `/Game/AIPhases/Blueprints/Turns/Enums/E_Phase` Phase))))

(event `PlayMontage`
  (params (MontageToPlay :type "AnimMontage Object Reference"))
  (`|ExecutionSequence`
    (:`then_0`
      (`self.bShowDebug?`
        (:`then`
          (`KismetSystemLibrary.PrintString` "BP_Character_Unit - EVENT Play Montage" true true (struct :`G` 0.66 :`B` 1.0 :`A` 1.0) 3.0))
        (:`else`)))
    (:`then_1`
      (`self.As BP Character Unit`
        (:`then`
          _)
        (:`else`
          (bind _asbp_character_unit (cast `/Game/AIPhases/Blueprints/Units/BP_Character_Unit` (`self.K2_GetPawn`)))
          (set `self.As BP Character Unit` _asbp_character_unit)))
      (`/Game/AIPhases/Blueprints/Units/BP_Character_Unit.MULTIPlayMontage` (`self.As BP Character Unit`) MontageToPlay))))

(event `PreperationActionUpdate`
  (params (ActionData :type "/Game/AIPhases/Blueprints/Action/Data/PDA_Action Object Reference"))
  (`|ExecutionSequence`
    (:`then_0`
      (`self.bShowDebug?`
        (:`then`
          (`KismetSystemLibrary.PrintString` "BP_Character_Unit - EVENT Preperation Action Update" true true (struct :`G` 0.66 :`B` 1.0 :`A` 1.0) 3.0))
        (:`else`)))
    (:`then_1`
      (set `self.PlanningActionData` ActionData))))

(event `MoveTo`
  (params (Location :type "Vector Structure"))
  (`|ExecutionSequence`
    (:`then_0`
      (`self.bShowDebug?`
        (:`then`
          (`KismetSystemLibrary.PrintString` "BP_Character_Unit - EVENT MoveTo" true true (struct :`G` 0.66 :`B` 1.0 :`A` 1.0) 3.0))
        (:`else`)))
    (:`then_1`
      (`self.As BP Character Unit`
        (:`then`
          _)
        (:`else`
          (bind _asbp_character_unit (cast `/Game/AIPhases/Blueprints/Units/BP_Character_Unit` (`self.K2_GetPawn`)))
          (set `self.As BP Character Unit` _asbp_character_unit)))
      (`/Game/AIPhases/Blueprints/Units/BP_Character_Unit.MultiMoveTo` (`self.As BP Character Unit`) Location))))

(event `DashActionUpdate`
  (params (DashActionData :type "/Game/AIPhases/Blueprints/Action/Data/PDA_Action Object Reference"))
  (`|ExecutionSequence`
    (:`then_0`
      (`self.bShowDebug?`
        (:`then`
          (`KismetSystemLibrary.PrintString` "BP_Character_Unit - EVENT Dash Action Update" true true (struct :`G` 0.66 :`B` 1.0 :`A` 1.0) 3.0))
        (:`else`)))
    (:`then_1`
      (set `self.DashActionData` DashActionData))))

(event `CombatActionUpdate`
  (params (CombatActionData :type "/Game/AIPhases/Blueprints/Action/Data/PDA_Action Object Reference"))
  (`|ExecutionSequence`
    (:`then_0`
      (`self.bShowDebug?`
        (:`then`
          (`KismetSystemLibrary.PrintString` "BP_Character_Unit - EVENT Combat Action Update" true true (struct :`G` 0.66 :`B` 1.0 :`A` 1.0) 3.0))
        (:`else`)))
    (:`then_1`
      (set `self.CombatActionData` CombatActionData))))

(event `AITurnStart`
  (params (Phase :type "/Game/AIPhases/Blueprints/Turns/Enums/E_Phase Enum" :default "NewEnumerator6"))
  (if (not (`|EnumEquality` (`self.Command`) "NewEnumerator2"))
    (`StateTreeComponent.SendStateTreeEvent` (`self.StateTreeAI_Melee`) (make `StateTreeEvent` (select `/Game/AIPhases/Blueprints/Turns/Enums/E_Phase` Phase :`NewEnumerator0` (struct :`TagName` "Phase.Planning") :`NewEnumerator3` (struct :`TagName` "Phase.Combat") :`NewEnumerator4` (struct :`TagName` "Phase.Movement") :!type "GameplayTag Structure")))))

(event `MovementActionUpdate`
  (params (MovementActionData :type "/Game/AIPhases/Blueprints/Action/Data/PDA_Action Object Reference"))
  (`|ExecutionSequence`
    (:`then_0`
      (`self.bShowDebug?`
        (:`then`
          (`KismetSystemLibrary.PrintString` "BP_Character_Unit - EVENT Movement Action Update" true true (struct :`G` 0.66 :`B` 1.0 :`A` 1.0) 3.0))
        (:`else`)))
    (:`then_1`
      (set `self.MovementActionData` MovementActionData))))

(event `DeathActionUpdate`
  (params (DeathActionData :type "/Game/AIPhases/Blueprints/Action/Data/PDA_Action Object Reference"))
  (`|ExecutionSequence`
    (:`then_0`
      (`self.bShowDebug?`
        (:`then`
          (`KismetSystemLibrary.PrintString` "BP_Character_Unit - EVENT Death Action Update" true true (struct :`G` 0.66 :`B` 1.0 :`A` 1.0) 3.0))
        (:`else`)))
    (:`then_1`
      (set `self.DeathActionData` DeathActionData))))

(fn `UserConstructionScript`)