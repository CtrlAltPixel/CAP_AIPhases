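; BP_GM_AIPhases is the game mode for AIPhases, tracking connected players and spawning their characters.
; Login and logout events add and remove entries in the AllPlayerControllers list.
; A spawn event creates a BP_Character_AIPhases_Player at the first PlayerStart found, passing the requesting BP_PC_AIPhases as CommandController.
; BeginPlay binds a character-death handler, which is currently empty.
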(event `self.ReceiveBeginPlay`
  (add `self.OnCharacterDied` (delegate `EventOnCharacterDied`)))

(event `EventOnCharacterDied` :!signature `self.OnCharacterDied`
  (params (NewParam :type "Character Object Reference")))

(event `self.K2_PostLogin`
  (params (NewPlayer :type "PlayerController Object Reference"))
  (`KismetArrayLibrary.Array_Add` (`self.AsAllPlayerControllers`) NewPlayer))

(event `self.K2_OnLogout`
  (params (ExitingController :type "Controller Object Reference"))
  (bind _asplayer_controller (cast `PlayerController` ExitingController))
  (`KismetArrayLibrary.Array_RemoveItem` (`self.AsAllPlayerControllers`) _asplayer_controller))

(event `EventSpawnPlayerCharacter`
  (params (PlayerController :type "PlayerController Object Reference"))
  (bind _asbp_pc_aiphases (cast `/Game/AIPhases/Player/Controller/BP_PC_AIPhases` PlayerController))
  (bind _outactors (`GameplayStatics.GetAllActorsOfClass` "/Script/Engine.PlayerStart"))
  (`|SpawnActorFromClass` "/Game/AIPhases/Characters/Player/BP_Character_AIPhases_Player.BP_Character_AIPhases_Player_C" (`self.GetTransform` (`|GetArrayItem` _outactors)) "Undefined" "MultiplyWithRoot" null _asbp_pc_aiphases null))

(fn `UserConstructionScript`)