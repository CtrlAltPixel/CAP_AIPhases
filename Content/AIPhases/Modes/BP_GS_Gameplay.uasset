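; BP_GS_Gameplay is a work-in-progress game state for a turn-based match with Planning, Preperation, Dash, Combat, Movement and Respawn phases.
; Chained events drive match, turn, phase and action start and end, branching on the replicated Phase.
; Planning starts a ready timer, other phases call action or spawn queue builders, and turn end checks kill count.
; Most helpers are stubs or incomplete, including phase advancing, queue ordering, animation and scoreboard.
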(event `self.ReceiveBeginPlay`
  (`|ExecutionSequence`
    (:`then_0`
      (if (`self.bShowDebug?`)
        (`KismetSystemLibrary.PrintString` "BP_GS_Gameplay - EVENT Begin Play" true true (struct :`G` 0.66 :`B` 1.0 :`A` 1.0) 3.0)))))

(event `EventGameStateMatchStart`
  (`|ExecutionSequence`
    (:`then_0`
      (if (`self.bShowDebug?`)
        (`KismetSystemLibrary.PrintString` "BP_GS_Gameplay - EVENT MatchStart" true true (struct :`G` 0.66 :`B` 1.0 :`A` 1.0) 3.0)))
    (:`then_1`
      (`self.StartMatchTimer`)
      (`self.EventGameStateTurnStart`))))

(event `EventGameStateMatchEnd`
  (`|ExecutionSequence`
    (:`then_0`
      (if (`self.bShowDebug?`)
        (`KismetSystemLibrary.PrintString` "BP_GS_Gameplay - EVENT MatchEnd" true true (struct :`G` 0.66 :`B` 1.0 :`A` 1.0) 3.0)))
    (:`then_1`
      (`self.ShowScoreboard`))))

(event `EventGameStateTurnStart`
  (`|ExecutionSequence`
    (:`then_0`
      (if (`self.bShowDebug?`)
        (`KismetSystemLibrary.PrintString` "BP_GS_Gameplay - EVENT Turn Start" true true (struct :`G` 0.66 :`B` 1.0 :`A` 1.0) 3.0)))
    (:`then_1`
      (`self.TurnDetails`)
      (`self.EnableActionBar`)
      (`self.StartReadyTimer`)
      (`self.EventGameStatePhaseStart`))))

(event `EventGameStateTurnEnd`
  (`|ExecutionSequence`
    (:`then_0`
      (if (`self.bShowDebug?`)
        (`KismetSystemLibrary.PrintString` "BP_GS_Gameplay - EVENT Turn End" true true (struct :`G` 0.66 :`B` 1.0 :`A` 1.0) 3.0)))
    (:`then_1`
      (bind _ismaxkills_ (`self.QueryKillCount`))
      (if _ismaxkills_
        (`self.EventGameStateMatchEnd`)
        (else
          (`self.EventGameStateTurnStart`))))))

(event `EventGameStatePhaseStart`
  (`|ExecutionSequence`
    (:`then_0`
      (if (`self.bShowDebug?`)
        (`KismetSystemLibrary.PrintString` "BP_GS_Gameplay - EVENT PhaseStart" true true (struct :`G` 0.66 :`B` 1.0 :`A` 1.0) 3.0)))
    (:`then_1`
      (switch `/Game/AIPhases/Modes/Enums/E_Phase` (`self.Phase`)
        (:`NewEnumerator0`
          (`self.FocusCamera`)
          (`self.StartReadyTimer`))
        (:`NewEnumerator1`
          (`self.CreateActionQue`)
          (`self.OrderActionQue`)
          (`self.EventGameStateActionStart`))
        (:`NewEnumerator2`
          (`self.CreateActionQue`)
          (`self.OrderActionQue`)
          (`self.EventGameStateActionStart`))
        (:`NewEnumerator3`
          (`self.CreateActionQue`)
          (`self.OrderActionQue`)
          (`self.EventGameStateActionStart`))
        (:`NewEnumerator4`
          (`self.CreateActionQue`)
          (`self.OrderActionQue`)
          (`self.EventGameStateActionStart`))
        (:`NewEnumerator5`
          (`self.CreateSpawnQue`)
          (`self.OrderActionQue`)
          (`self.EventGameStateActionStart`))))))

(event `EventGameStatePhaseEnd`
  (`|ExecutionSequence`
    (:`then_0`
      (if (`self.bShowDebug?`)
        (`KismetSystemLibrary.PrintString` "BP_GS_Gameplay - EVENT Phase End" true true (struct :`G` 0.66 :`B` 1.0 :`A` 1.0) 3.0)))
    (:`then_1`
      (switch `/Game/AIPhases/Modes/Enums/E_Phase` (`self.Phase`)
        (:`NewEnumerator0`
          (`self.DisableActionBar`)
          (`KismetSystemLibrary.K2_ClearAndInvalidateTimerHandle` (`self.ReayTimer`))
          (`self.AdvancePhase`))
        (:`NewEnumerator1`
          (`self.AdvancePhase`))
        (:`NewEnumerator2`
          (`self.AdvancePhase`))
        (:`NewEnumerator3`
          (`self.AdvancePhase`))
        (:`NewEnumerator4`
          (`self.AdvancePhase`))
        (:`NewEnumerator5`
          (`self.EventGameStateTurnEnd`))))))

(event `EventGameStateActionStart`
  (`|ExecutionSequence`
    (:`then_0`
      (if (`self.bShowDebug?`)
        (`KismetSystemLibrary.PrintString` "BP_GS_Gameplay - EVENT ActionStart" true true (struct :`G` 0.66 :`B` 1.0 :`A` 1.0) 3.0)))
    (:`then_1`
      (bind _bishidden_ (`self.IsHiddenAction?`))
      (if _bishidden_
        (`self.ShowHiddenMessage`)
        (else
          (`self.FocusCamera`)))
      (`self.AnimateUnit`)
      (`self.EventGameStateActionEnd`))))

(event `EventGameStateActionEnd`
  (`|ExecutionSequence`
    (:`then_0`
      (if (`self.bShowDebug?`)
        (`KismetSystemLibrary.PrintString` "BP_GS_Gameplay - EVENT ActionEnd" true true (struct :`G` 0.66 :`B` 1.0 :`A` 1.0) 3.0)))
    (:`then_1`
      (bind _bisempty_ (`self.QueryActionQue`))
      (if _bisempty_
        (`self.EventGameStatePhaseEnd`)
        (else
          (`self.EventGameStateActionStart`))))))

(fn `AdvancePhase`)

(fn `AdvanceTurn`)

(fn `AnimateUnit`)

(fn `CreateActionQue`
  (returns (Units :type "Array of /Game/AIPhases/Characters/BP_Character_Unit Object Reference"))
  (locals (Local_UnitsToAction :type "Array of /Game/AIPhases/Characters/BP_Character_Unit Object Reference"))
  (bind _outactors (`GameplayStatics.GetAllActorsOfClass` "/Game/AIPhases/Characters/BP_Character_Unit.BP_Character_Unit_C"))
  (for _ _outactors
    (cast `/Game/AIPhases/Characters/AI/BP_AIController_Gameplay` (`AIBlueprintHelperLibrary.GetAIController` null)))
  (return (`local.Local_UnitsToAction`)))

(fn `CreateSpawnQue`
  (locals (Local_UnitsToAction :type "Array of /Game/AIPhases/Characters/BP_Character_Unit Object Reference"))
  (`GameplayStatics.GetAllActorsOfClass` "BP_GS_Gameplay_C"))

(fn `DisableActionBar`
  (returns (`bAllLocked?` :type Boolean))
  (for _array_element (`self.PlayerArray`)
    (`self.As BP PC AIPhases`
      (:`then`)
      (:`else`
        (bind _asbp_pc_aiphases (cast `/Game/AIPhases/Player/Controller/BP_PC_AIPhases` (`PlayerState.GetPlayerController` _array_element)))
        (set `self.As BP PC AIPhases` _asbp_pc_aiphases))))
  (return true))

(fn `EnableActionBar`
  (for _array_element (`self.PlayerArray`)
    (`self.As BP PC AIPhases`
      (:`then`)
      (:`else`
        (bind _asbp_pc_aiphases (cast `/Game/AIPhases/Player/Controller/BP_PC_AIPhases` (`PlayerState.GetPlayerController` _array_element)))
        (set `self.As BP PC AIPhases` _asbp_pc_aiphases)))))

(fn `FocusCamera`)

(fn `IsHiddenAction?`
  (returns (`bIsHidden?` :type Boolean))
  (return false))

(fn `OnRep_Phase`
  (`self.OnPhaseChange` (`self.Phase`)))

(fn `OrderActionQue`)

(fn `QueryActionQue`
  (returns (`bIsEmpty?` :type Boolean))
  (return (`KismetArrayLibrary.Array_IsEmpty` (`self.ActionQue`))))

(fn `QueryKillCount`
  (returns (`IsMaxKills?` :type Boolean))
  (return (>= 0 (`self.Setting_MaxKills`))))

(fn `ShowHiddenMessage`)

(fn `ShowScoreboard`)

(fn `StartMatchTimer`
  (bind _returnvalue (`KismetSystemLibrary.K2_SetTimer` null "" 1.0 true))
  (set `self.MatchTimer` _returnvalue))

(fn `StartReadyTimer`
  (bind _returnvalue (`KismetSystemLibrary.K2_SetTimer` null "" 1.0 true))
  (set `self.ReayTimer` _returnvalue))

(fn `TurnDetails`
  (set `self.TurnCount` (+ (`self.TurnCount`) 1)))

(fn `UserConstructionScript`)