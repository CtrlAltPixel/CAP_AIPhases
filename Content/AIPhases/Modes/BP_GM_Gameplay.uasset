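; Gameplay game mode for AIPhases that maintains a list of connected player controllers, adding them on login and removing them on logout.
; BeginPlay binds a character-died handler, but that handler is empty.
; The unit spawn event only validates the PlayerState.
; Two disconnected node chains, which never run, spawn player characters and possess them with gameplay AI controllers.
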(event `self.ReceiveBeginPlay`
  (add `self.OnCharacterDied` (delegate `EventOnCharacterDied`)))

(event `EventOnCharacterDied` :!signature `self.OnCharacterDied`
  (params (Character :type "Character Object Reference")))

(event `self.K2_PostLogin`
  (params (NewPlayer :type "PlayerController Object Reference"))
  (`KismetArrayLibrary.Array_Add` (`self.AsAllPlayerControllers`) NewPlayer))

(event `self.K2_OnLogout`
  (params (ExitingController :type "Controller Object Reference"))
  (bind _asplayer_controller (cast `PlayerController` ExitingController))
  (`KismetArrayLibrary.Array_RemoveItem` (`self.AsAllPlayerControllers`) _asplayer_controller))

(event `EventGameModeSpawnUnit`
  (params (PlayerState :type "PlayerState Object Reference"))
  (`/Engine/EditorBlueprintResources/StandardMacros.IsValid` PlayerState))

(fn `UserConstructionScript`)