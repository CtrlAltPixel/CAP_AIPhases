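; Player controller for the custom lobby, handling mouse input setup and team slot requests.
; On BeginPlay, the local controller enables the cursor, click and mouse-over events, and caches BP_HUD_CustomLobby.
; RequestTeam passes its PlayerState, index and team to HandlePlayerRequestTeam on a lazily cached BP_GS_CustomLobby.
; The Blue, Red and Spectator HUD update events only print debug text and cache the HUD, without refreshing anything.
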(event `self.ReceiveBeginPlay`
  (`|ExecutionSequence`
    (:`then_0`
      (`self.bShowDebug?`
        (:`then`
          (`KismetSystemLibrary.PrintString` "BP_PC_CustomLobby - EVENT Begin Play" true true (struct :`G` 0.66 :`B` 1.0 :`A` 1.0) 3.0))
        (:`else`)))
    (:`then_1`
      (if (`self.IsLocalPlayerController`)
        (`self.HUD`)))))

(event `HUD`
  (`|ExecutionSequence`
    (:`then_0`
      (`self.bShowDebug?`
        (:`then`
          (`KismetSystemLibrary.PrintString` "BP_PC_CustomLobby - EVENT HUD" true true (struct :`G` 0.66 :`B` 1.0 :`A` 1.0) 3.0))
        (:`else`)))
    (:`then_1`
      (set `self.bShowMouseCursor` true)
      (set `self.bEnableClickEvents` true)
      (set `self.bEnableMouseOverEvents` true))
    (:`then_2`
      (`self.As BP HUD Custom Lobby`
        (:`then`)
        (:`else`
          (bind _asbp_hud_custom_lobby (cast `/Game/AIPhases/CustomLobby/HUD/BP_HUD_CustomLobby` (`self.GetHUD`)))
          (set `self.As BP HUD Custom Lobby` _asbp_hud_custom_lobby))))))

(event `HUDUpdateTeamBlue`
  (`|ExecutionSequence`
    (:`then_0`
      (`self.bShowDebug?`
        (:`then`
          (`KismetSystemLibrary.PrintString` "BP_PC_CustomLobby - EVENT Client Refresh Team Blue" true true (struct :`G` 0.66 :`B` 1.0 :`A` 1.0) 3.0))
        (:`else`)))
    (:`then_1`
      (`self.As BP HUD Custom Lobby`
        (:`then`)
        (:`else`
          (bind _asbp_hud_custom_lobby (cast `/Game/AIPhases/CustomLobby/HUD/BP_HUD_CustomLobby` (`self.GetHUD`)))
          (set `self.As BP HUD Custom Lobby` _asbp_hud_custom_lobby))))))

(event `HUDUpdateTeamRed`
  (`|ExecutionSequence`
    (:`then_0`
      (`self.bShowDebug?`
        (:`then`
          (`KismetSystemLibrary.PrintString` "BP_PC_CustomLobby - EVENT Client Refresh Team Red" true true (struct :`G` 0.66 :`B` 1.0 :`A` 1.0) 3.0))
        (:`else`)))
    (:`then_1`
      (`self.As BP HUD Custom Lobby`
        (:`then`)
        (:`else`
          (bind _asbp_hud_custom_lobby (cast `/Game/AIPhases/CustomLobby/HUD/BP_HUD_CustomLobby` (`self.GetHUD`)))
          (set `self.As BP HUD Custom Lobby` _asbp_hud_custom_lobby))))))

(event `HUDUpdateTeamSpectator`
  (`|ExecutionSequence`
    (:`then_0`
      (`self.bShowDebug?`
        (:`then`
          (`KismetSystemLibrary.PrintString` "BP_PC_CustomLobby - EVENT Client Refresh Team Spectator" true true (struct :`G` 0.66 :`B` 1.0 :`A` 1.0) 3.0))
        (:`else`)))
    (:`then_1`
      (`self.As BP HUD Custom Lobby`
        (:`then`)
        (:`else`
          (bind _asbp_hud_custom_lobby (cast `/Game/AIPhases/CustomLobby/HUD/BP_HUD_CustomLobby` (`self.GetHUD`)))
          (set `self.As BP HUD Custom Lobby` _asbp_hud_custom_lobby))))))

(event `RequestTeam`
  (params (Index :type Integer) (Team :type "/Game/AIPhases/Blueprints/Team/Enum/E_Team Enum" :default "NewEnumerator0"))
  (`|ExecutionSequence`
    (:`then_0`
      (`self.bShowDebug?`
        (:`then`
          (`KismetSystemLibrary.PrintString` "BP_PC_CustomLobby - EVENT Request" true true (struct :`G` 0.66 :`B` 1.0 :`A` 1.0) 3.0))
        (:`else`)))
    (:`then_1`
      (`self.As BP GS Custom Lobby`
        (:`then`
          _)
        (:`else`
          (bind _asbp_gs_custom_lobby (cast `/Game/AIPhases/CustomLobby/Mode/BP_GS_CustomLobby` (`GameplayStatics.GetGameState`)))
          (set `self.As BP GS Custom Lobby` _asbp_gs_custom_lobby)))
      (`/Game/AIPhases/CustomLobby/Mode/BP_GS_CustomLobby.HandlePlayerRequestTeam` (`self.As BP GS Custom Lobby`) (`self.PlayerState`) Index Team))))

(fn `UserConstructionScript`)