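; Custom lobby game state that tracks players in Blue, Red and Spectator slot arrays.
; A team request moves the player only if QueryTeamIndex returns true, which as written means the requested slot already holds a valid entry.
; The move removes the player from the old array, writes the new slot and updates BP_PS_CustomLobby's team.
; Each array's RepNotify has the local BP_PC_CustomLobby refresh that team.
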(event `self.ReceiveBeginPlay`
  (`|ExecutionSequence`
    (:`then_0`
      (`self.bShowDebug?`
        (:`then`
          (`KismetSystemLibrary.PrintString` "WBP_GS_Lobby - EVENT BeginPlay" true true (struct :`G` 0.66 :`B` 1.0 :`A` 1.0) 3.0))
        (:`else`)))))

(event `HandlePlayerRequestTeam`
  (params (PlayerState :type "PlayerState Object Reference") (Index :type Integer) (Team :type "/Game/AIPhases/Blueprints/Team/Enum/E_Team Enum" :default "NewEnumerator0"))
  (`|ExecutionSequence`
    (:`then_0`
      (`self.bShowDebug?`
        (:`then`
          (`KismetSystemLibrary.PrintString` "WBP_GS_Lobby - EVENT BeginPlay" true true (struct :`G` 0.66 :`B` 1.0 :`A` 1.0) 3.0))
        (:`else`)))
    (:`then_1`
      (bind _bisvalid (`self.QueryTeamIndex` Team Index))
      (if _bisvalid
        (`self.RemovePlayerFromTeam` PlayerState)
        (`self.AddPlayerToTeam` PlayerState Index Team)))))

(fn `AddPlayerToTeam`
  (params (Playerstate :type "PlayerState Object Reference (by ref)") (Index :type Integer) (Team :type "/Game/AIPhases/Blueprints/Team/Enum/E_Team Enum" :default "NewEnumerator0"))
  (`|ExecutionSequence`
    (:`then_0`
      (`self.bShowDebug?`
        (:`then`
          (`KismetSystemLibrary.PrintString` "WBP_GS_Lobby - FUNCTION Add Player To Team" true true (struct :`G` 0.66 :`B` 1.0 :`A` 1.0) 3.0))
        (:`else`)))
    (:`then_1`
      (switch `/Game/AIPhases/Blueprints/Team/Enum/E_Team` (`local.Team`)
        (:`NewEnumerator1`
          (`KismetArrayLibrary.Array_Set` (`self.TeamBlue`) (`local.Index`) (`local.Playerstate`) true))
        (:`NewEnumerator3`
          (`KismetArrayLibrary.Array_Set` (`self.TeamSpectators`) (`local.Index`) (`local.Playerstate`) true))
        (:`NewEnumerator4`
          (`KismetArrayLibrary.Array_Set` (`self.TeamRed`) (`local.Index`) (`local.Playerstate`) true))))
    (:`then_2`
      (bind _asbp_ps_custom_lobby (cast `/Game/AIPhases/CustomLobby/Player/BP_PS_CustomLobby` (`local.Playerstate`)))
      (`/Game/AIPhases/CustomLobby/Player/BP_PS_CustomLobby.SetTeam` _asbp_ps_custom_lobby (`local.Team`)))))

(fn `OnRep_TeamBlue`
  (bind _returnvalue (`GameplayStatics.GetPlayerController` 0))
  (`|ExecutionSequence`
    (:`then_0`
      (`self.bShowDebug?`
        (:`then`
          (`KismetSystemLibrary.PrintString` "WBP_GS_Lobby - ONREP Team Blue" true true (struct :`G` 0.66 :`B` 1.0 :`A` 1.0) 3.0))
        (:`else`)))
    (:`then_1`
      (if (`Controller.IsLocalController` _returnvalue)
        (bind _asbp_pc_custom_lobby (cast `/Game/AIPhases/CustomLobby/Player/BP_PC_CustomLobby` _returnvalue))
        (`/Game/AIPhases/CustomLobby/Player/BP_PC_CustomLobby.ClientRefreshTeamBlue` _asbp_pc_custom_lobby)))))

(fn `OnRep_TeamRed`
  (bind _returnvalue (`GameplayStatics.GetPlayerController` 0))
  (`|ExecutionSequence`
    (:`then_0`
      (`self.bShowDebug?`
        (:`then`
          (`KismetSystemLibrary.PrintString` "WBP_GS_Lobby - ONREP Team Red" true true (struct :`G` 0.66 :`B` 1.0 :`A` 1.0) 3.0))
        (:`else`)))
    (:`then_1`
      (if (`Controller.IsLocalController` _returnvalue)
        (bind _asbp_pc_custom_lobby (cast `/Game/AIPhases/CustomLobby/Player/BP_PC_CustomLobby` _returnvalue))
        (`/Game/AIPhases/CustomLobby/Player/BP_PC_CustomLobby.ClientRefreshTeamRed` _asbp_pc_custom_lobby)))))

(fn `OnRep_TeamSpectators`
  (bind _returnvalue (`GameplayStatics.GetPlayerController` 0))
  (`|ExecutionSequence`
    (:`then_0`
      (`self.bShowDebug?`
        (:`then`
          (`KismetSystemLibrary.PrintString` "WBP_GS_Lobby - ONREP Team Spectator" true true (struct :`G` 0.66 :`B` 1.0 :`A` 1.0) 3.0))
        (:`else`)))
    (:`then_1`
      (if (`Controller.IsLocalController` _returnvalue)
        (bind _asbp_pc_custom_lobby (cast `/Game/AIPhases/CustomLobby/Player/BP_PC_CustomLobby` _returnvalue))
        (`/Game/AIPhases/CustomLobby/Player/BP_PC_CustomLobby.ClientRefreshTeamSpectator` _asbp_pc_custom_lobby)))))

(fn `QueryTeamIndex`
  (params (Selection :type "/Game/AIPhases/Blueprints/Team/Enum/E_Team Enum" :default "NewEnumerator0") (Index :type Integer))
  (returns (bIsValid :type Boolean))
  (`|ExecutionSequence`
    (:`then_0`
      (`self.bShowDebug?`
        (:`then`
          (`KismetSystemLibrary.PrintString` "WBP_GS_Lobby - FUNCTION QueryTeam" true true (struct :`G` 0.66 :`B` 1.0 :`A` 1.0) 3.0))
        (:`else`)))
    (:`then_1`
      (switch `/Game/AIPhases/Blueprints/Team/Enum/E_Team` Selection
        (:`NewEnumerator1`
          (`/Engine/EditorBlueprintResources/StandardMacros.IsValid` (`|GetArrayItem` (`self.TeamBlue`) (`local.Index`))
            (:`Is Valid`
              (return true))
            (:`Is Not Valid`
              (return false))))
        (:`NewEnumerator3`
          (`/Engine/EditorBlueprintResources/StandardMacros.IsValid` (`|GetArrayItem` (`self.TeamSpectators`) (`local.Index`))
            (:`Is Valid`
              (return true))
            (:`Is Not Valid`
              (return false))))
        (:`NewEnumerator4`
          (`/Engine/EditorBlueprintResources/StandardMacros.IsValid` (`|GetArrayItem` (`self.TeamRed`) (`local.Index`))
            (:`Is Valid`
              (return true))
            (:`Is Not Valid`
              (return false))))))))

(fn `RemovePlayerFromTeam`
  (params (PlayerState :type "PlayerState Object Reference"))
  (returns (bSuccess :type Boolean))
  (`|ExecutionSequence`
    (:`then_0`
      (`self.bShowDebug?`
        (:`then`
          (`KismetSystemLibrary.PrintString` "WBP_GS_Lobby - FUNCTION Add Player To Team" true true (struct :`G` 0.66 :`B` 1.0 :`A` 1.0) 3.0))
        (:`else`)))
    (:`then_1`
      (bind _asbp_ps_custom_lobby (cast `/Game/AIPhases/CustomLobby/Player/BP_PS_CustomLobby` (`local.PlayerState`)))
      (switch `/Game/AIPhases/Blueprints/Team/Enum/E_Team` (`/Game/AIPhases/CustomLobby/Player/BP_PS_CustomLobby.Team` _asbp_ps_custom_lobby)
        (:`NewEnumerator1`
          (bind _returnvalue (`KismetArrayLibrary.Array_RemoveItem` (`self.TeamBlue`) (`local.PlayerState`)))
          (return _returnvalue))
        (:`NewEnumerator3`
          (bind _returnvalue_2 (`KismetArrayLibrary.Array_RemoveItem` (`self.TeamSpectators`) (`local.PlayerState`)))
          (return _returnvalue_2))
        (:`NewEnumerator4`
          (bind _returnvalue_3 (`KismetArrayLibrary.Array_RemoveItem` (`self.TeamRed`) (`local.PlayerState`)))
          (return _returnvalue_3))))))

(fn `UserConstructionScript`)