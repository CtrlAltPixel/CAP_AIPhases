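; Player controller for AIPhases that drives a camera pawn and handles cursor-based character selection.
; On BeginPlay the local controller adds camera and interact Enhanced Input contexts, caches its HUD and camera pawn, and enables mouse events.
; Camera input forwards to the pawn, while primary interact stores the actor under the cursor from a channel trace, then calls the selection update, whose wiring passes no actor.
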(event `self.ReceiveBeginPlay`
  (bind _returnvalue (subsystem `EnhancedInputLocalPlayerSubsystem`))
  ;[0.05098 0.05098 0.05098] Add Mapping Context
  (if (`self.IsLocalPlayerController`)
    (`/Engine/EditorBlueprintResources/StandardMacros.IsValid` _returnvalue
      (:`Is Valid`
        (`EnhancedInputSubsystemInterface.AddMappingContext` _returnvalue "/Game/AIPhases/Input/IMC_Camera.IMC_Camera" 0 (struct))
        (`EnhancedInputSubsystemInterface.AddMappingContext` _returnvalue "/Game/AIPhases/Input/IMC_Interact.IMC_Interact" 0 (struct))
        (`self.InitCasts`)
        (`WidgetBlueprintLibrary.SetInputMode_GameAndUIEx` self null)
        (set `self.CurrentClickTraceChannel` "ECC_GameTraceChannel1")
        (set `self.bEnableClickEvents` true)
        (set `self.bEnableMouseOverEvents` true)))))

(event `EnhancedInput|/Game/AIPhases/Input/Actions/IA_PrimaryInteract`
  (params (ActionValue :type Boolean) (ElapsedSeconds :type "Float (double-precision)") (TriggeredSeconds :type "Float (double-precision)") (InputAction :type "InputAction Object Reference" :default "/Game/AIPhases/Input/Actions/IA_PrimaryInteract.IA_PrimaryInteract"))
  (bind (_hit _hitactor) (`self.GatActorUnderCursorByChannel` "TraceTypeQuery3"))
  (:`Triggered`
    (if (`GameplayStatics.ObjectIsA` (`self.AsInteractActor`))
      (`self.UpdateSelectedCharacter` null)))
  (:`Started`
    (if _hit
      (set `self.AsInteractActor` _hitactor))))

(event `EnhancedInput|/Game/AIPhases/Input/Actions/IA_CameraMove`
  (params (ActionValue :type "Vector2D Structure") (ElapsedSeconds :type "Float (double-precision)") (TriggeredSeconds :type "Float (double-precision)") (InputAction :type "InputAction Object Reference" :default "/Game/AIPhases/Input/Actions/IA_CameraMove.IA_CameraMove"))
  (:`Triggered`
    (bind _as_bp_pawn_camera (`self.As BP Pawn Camera`)
      (:`then`
        (`/Game/AIPhases/Player/Camera/BP_Pawn_Camera.CameraMove` _as_bp_pawn_camera ActionValue_X ActionValue_Y))
      (:`else`))))

(fn `GatActorUnderCursorByChannel`
  (params (TraceChannel :type "ETraceTypeQuery Enum" :default "TraceTypeQuery1"))
  (returns (Hit :type Boolean) (HitActor :type "Actor Object Reference"))
  (bind (_bblockinghit _binitialoverlap _time _distance _location _impactpoint _normal _impactnormal _physmat _hitactor) (`GameplayStatics.BreakHitResult` (`self.GetHitResultUnderCursorByChannel` TraceChannel)))
  (return _bblockinghit _hitactor))

(fn `InitCasts`
  (bind _asbp_hud_aiphases (cast `/Game/AIPhases/UI/HUD/BP_HUD_AIPhases` (`self.GetHUD`)))
  (set `self.As BP HUD AIPhases` _asbp_hud_aiphases)
  (bind _asbp_pawn_camera (cast `/Game/AIPhases/Player/Camera/BP_Pawn_Camera` (`self.K2_GetPawn`)))
  (set `self.As BP Pawn Camera` _asbp_pawn_camera))

(fn `UpdateSelectedCharacter`
  (params (Actor :type "Actor Object Reference"))
  (bind _asbp_character_aiphases (cast `/Game/AIPhases/Characters/BP_Character_AIPhases` Actor))
  (set `self.AsSelectedBP Character AIPhases` _asbp_character_aiphases))

(fn `UserConstructionScript`)