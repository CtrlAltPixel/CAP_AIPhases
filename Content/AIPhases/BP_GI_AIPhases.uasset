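; BP_GI_AIPhases is a Blueprint, apparently a Game Instance, that handles hosting, finding and joining multiplayer sessions.
; CreateSession opens an eight-slot session and, on success, loads the custom lobby level as a listen server.
; FindSession refills FoundSessions from the immediate output rather than a success callback, while JoinSession joins a supplied search result.
; Each event can print a debug message, gated by a ShowDebug validity check.
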(event `CreateSession`
  (`|ExecutionSequence`
    (:`then_0`
      (`self.bShowDebug`
        (:`then`
          (`KismetSystemLibrary.PrintString` "BP_GI_AIPhases - EVENT HostSession" true true (struct :`G` 0.66 :`B` 1.0 :`A` 1.0) 3.0))
        (:`else`)))
    (:`then_1`
      (`CreateSessionCallbackProxy.CreateSession` (`GameplayStatics.GetPlayerController` 0) 8
        (:`OnSuccess`
          (`GameplayStatics.OpenLevelBySoftObjectPtr` "/Game/AIPhases/CustomLobby/Map/LVL_CustomLobby.LVL_CustomLobby" true "?listen"))))))

(event `FindSession`
  (`|ExecutionSequence`
    (:`then_0`
      (`self.bShowDebug`
        (:`then`
          (`KismetSystemLibrary.PrintString` "BP_GI_AIPhases - EVENT FindSession Session" true true (struct :`G` 0.66 :`B` 1.0 :`A` 1.0) 3.0))
        (:`else`)))
    (:`then_1`
      (`KismetArrayLibrary.Array_Clear` (`self.FoundSessions`))
      (bind _results (`FindSessionsCallbackProxy.FindSessions` (`GameplayStatics.GetPlayerController` 0))
        (:`then`
          (set `self.FoundSessions` _results))))))

(event `JoinSession`
  (params (SearchResult :type "BlueprintSessionResult Structure (by ref)"))
  (`|ExecutionSequence`
    (:`then_0`
      (`self.bShowDebug`
        (:`then`
          (`KismetSystemLibrary.PrintString` "BP_GI_AIPhases - EVENT Join Session" true true (struct :`G` 0.66 :`B` 1.0 :`A` 1.0) 3.0))
        (:`else`)))
    (:`then_1`
      (`JoinSessionCallbackProxy.JoinSession` (`GameplayStatics.GetPlayerController` 0) SearchResult))))