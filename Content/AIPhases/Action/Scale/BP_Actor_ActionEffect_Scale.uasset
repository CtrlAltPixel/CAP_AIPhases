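; An AI phase action effect actor that resizes its target unit by a scale multiplier.
; When the action starts, it caches the unit's current actor scale, applies that scale times Scale, then immediately ends the action.
; The change is instant: a TL_Scale timeline exists but never runs, and nothing here restores the cached scale.
; An optional debug print logs the start under the older-looking name ActionEffect_Size.
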(event `self.EventActionStart`
  (bind _target_unit (`self.Target Unit`))
  (`|ExecutionSequence`
    (:`then_0`
      (if (`self.bShowDebug?`)
        (`KismetSystemLibrary.PrintString` "BP_Actor_ActionEffect_Size - EVENT Begin Play" true true (struct :`G` 0.66 :`B` 1.0 :`A` 1.0) 3.0)))
    (:`then_1`
      (set `self.CachedScale` (`self.GetActorScale3D` _target_unit))
      (`self.SetActorScale3D` _target_unit (* (`self.CachedScale`) (`self.Scale`)))
      (`self.EventActionEnd`))))

(fn `UserConstructionScript`
  (`parent.UserConstructionScript`))