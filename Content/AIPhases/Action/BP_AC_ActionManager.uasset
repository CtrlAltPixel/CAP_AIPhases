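; Base actor component for unit actions in the AI phases, with stub CanAddAction, ModifyActionValue and RemoveAction functions.
; On BeginPlay it multicasts the Data montage on its owning BP_Character_Unit, then modifies the value and fires the add event if CanAddAction passes.
; The add event caches the gameplay GameState, but its dispatcher call and end-play binding are unwired.
; The remove event calls OnActionRemove.
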(event `self.ReceiveBeginPlay`
  (bind _returnvalue (`self.GetOwner`))
  (`|ExecutionSequence`
    (:`then_0`
      (if (`self.bShowDebug?`)
        (`KismetSystemLibrary.PrintString` "BP_AC_Action - EVENT Begin Play" true true (struct :`G` 0.66 :`B` 1.0 :`A` 1.0) 3.0)))
    (:`then_1`
      (`/Engine/EditorBlueprintResources/StandardMacros.IsValid` _returnvalue
        (:`Is Valid`
          (bind _asbp_character_unit (cast `/Game/AIPhases/Characters/BP_Character_Unit` _returnvalue))
          (`/Game/AIPhases/Characters/BP_Character_Unit.MULTIPlayMontage` _asbp_character_unit (`/Game/AIPhases/Action/Data/PDA_Action.Montage` (`self.Data`)))
          (bind _bcanadd_ (`self.CanAddAction?`))
          (if _bcanadd_
            (`self.ModifyActionValue?`)
            (`self.EventActionAdd`)))))))

(event `EventActionAdd`
  (`|ExecutionSequence`
    (:`then_0`
      (if (`self.bShowDebug?`)
        (`KismetSystemLibrary.PrintString` "BP_AC_Action - EVENT Action ADD Effect" true true (struct :`G` 0.66 :`B` 1.0 :`A` 1.0) 3.0)))
    (:`then_1`
      (`self.As BP GS Gameplay`
        (:`then`)
        (:`else`
          (bind _asbp_gs_gameplay (cast `/Game/AIPhases/Modes/BP_GS_Gameplay` (`GameplayStatics.GetGameState`)))
          (bind _output_get (set `self.As BP GS Gameplay` _asbp_gs_gameplay)))))))

(event `EventActionRemove`
  (`|ExecutionSequence`
    (:`then_0`
      (if (`self.bShowDebug?`)
        (`KismetSystemLibrary.PrintString` "BP_AC_Action - EVENT Action Remove Effect" true true (struct :`G` 0.66 :`B` 1.0 :`A` 1.0) 3.0)))
    (:`then_1`
      (`self.OnActionRemove`))))

(fn `CanAddAction?`
  (returns (`bCanAdd?` :type Boolean)))

(fn `ModifyActionValue?`)

(fn `RemoveAction?`)