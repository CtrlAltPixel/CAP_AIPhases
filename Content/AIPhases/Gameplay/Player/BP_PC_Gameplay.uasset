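; Gameplay player controller that links camera pawn, HUD and the player's current unit.
; On local BeginPlay it adds camera and interact Enhanced Input contexts and enables mouse click and hover events.
; Start events cache the camera pawn and HUD; move input drives the camera, while unit and weapon updates feed the HUD.
; A RepNotify refreshes the HUD's unit; interaction is stubbed beside an under-cursor trace helper.
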(event `self.ReceiveBeginPlay`
  (bind _returnvalue (subsystem `EnhancedInputLocalPlayerSubsystem`))
  ;[0.05098 0.05098 0.05098] Add Mapping Context
  (if (`self.IsLocalPlayerController`)
    (`/Engine/EditorBlueprintResources/StandardMacros.IsValid` _returnvalue
      (:`Is Valid`
        (`EnhancedInputSubsystemInterface.AddMappingContext` _returnvalue "/Game/AIPhases/Gameplay/Player/Input/IMC_Camera.IMC_Camera" 0 (struct))
        (`EnhancedInputSubsystemInterface.AddMappingContext` _returnvalue "/Game/AIPhases/Gameplay/Player/Input/IMC_Interact.IMC_Interact" 0 (struct))
        (set `self.CurrentClickTraceChannel` "ECC_GameTraceChannel1")
        (set `self.bEnableClickEvents` true)
        (set `self.bEnableMouseOverEvents` true)))))

(event `CameraStart`
  (`|ExecutionSequence`
    (:`then_0`
      (`self.bShowDebug`
        (:`then`
          (`KismetSystemLibrary.PrintString` "BP_PC_Gameplay - EVENT Camera Start" true true (struct :`G` 0.66 :`B` 1.0 :`A` 1.0) 3.0))
        (:`else`)))
    (:`then_1`
      (`self.As BP Pawn Camera`
        (:`then`
          _)
        (:`else`
          (bind _asbp_pawn_camera (cast `/Game/AIPhases/Blueprints/Camera/BP_Pawn_Camera` (`self.K2_GetPawn`)))
          (set `self.As BP Pawn Camera` _asbp_pawn_camera)))
      (`self.SetViewTargetWithBlend` (`self.As BP Pawn Camera`)))))

(event `EnhancedInput|/Game/AIPhases/Gameplay/Player/Input/Actions/IA_Camera_Move`
  (params (ActionValue :type "Vector2D Structure") (ElapsedSeconds :type "Float (double-precision)") (TriggeredSeconds :type "Float (double-precision)") (InputAction :type "InputAction Object Reference" :default "/Game/AIPhases/Gameplay/Player/Input/Actions/IA_Camera_Move.IA_Camera_Move"))
  (:`Triggered`
    (bind _as_bp_pawn_camera (`self.As BP Pawn Camera`)
      (:`then`
        (`/Game/AIPhases/Blueprints/Camera/BP_Pawn_Camera.CameraMove` _as_bp_pawn_camera ActionValue_X ActionValue_Y))
      (:`else`))))

(event `EventHUDStart`
  (`|ExecutionSequence`
    (:`then_0`
      (`self.bShowDebug`
        (:`then`
          (`KismetSystemLibrary.PrintString` "BP_PC_Gameplay - EVENT Camera Start" true true (struct :`G` 0.66 :`B` 1.0 :`A` 1.0) 3.0))
        (:`else`)))
    (:`then_1`
      (`self.As BP_HUD_Gameplay`
        (:`then`)
        (:`else`
          (bind _asbp_hud_gameplay (cast `/Game/AIPhases/Gameplay/HUD/BP_HUD_Gameplay` (`self.GetHUD`)))
          (set `self.As BP_HUD_Gameplay` _asbp_hud_gameplay))))))

(event `InteractStart`
  (`|ExecutionSequence`
    (:`then_0`
      (`self.bShowDebug`
        (:`then`
          (`KismetSystemLibrary.PrintString` "BP_PC_Gameplay - EVENT Interact Start" true true (struct :`G` 0.66 :`B` 1.0 :`A` 1.0) 3.0))
        (:`else`)))))

(event `EnhancedInput|/Game/AIPhases/Gameplay/Player/Input/Actions/IA_Interact_Primary`
  (params (ActionValue :type Boolean) (ElapsedSeconds :type "Float (double-precision)") (TriggeredSeconds :type "Float (double-precision)") (InputAction :type "InputAction Object Reference" :default "/Game/AIPhases/Gameplay/Player/Input/Actions/IA_Interact_Primary.IA_Interact_Primary")))

(event `UnitUpdate`
  (params (Unit :type "/Game/AIPhases/Blueprints/Units/BP_Character_Unit Object Reference"))
  (`|ExecutionSequence`
    (:`then_0`
      (`self.bShowDebug`
        (:`then`
          (`KismetSystemLibrary.PrintString` "BP_PC_Gameplay - EVENT Update Unit" true true (struct :`G` 0.66 :`B` 1.0 :`A` 1.0) 3.0))
        (:`else`)))
    (:`then_1`
      (set `self.As BP_Character_Unit` Unit))
    (:`then_2`
      (bind _as_bp_hud_gameplay (`self.As BP_HUD_Gameplay`)
        (:`then`
          (`/Game/AIPhases/Gameplay/HUD/BP_HUD_Gameplay.UpdateUnit` _as_bp_hud_gameplay (`self.As BP_Character_Unit`)))
        (:`else`)))))

(event `WeaponUpdate`
  (params (WeaponData :type "/Game/AIPhases/Blueprints/Weapon/Data/PDA_Weapon Object Reference"))
  (`|ExecutionSequence`
    (:`then_0`
      (`self.bShowDebug`
        (:`then`
          (`KismetSystemLibrary.PrintString` "BP_PC_Gameplay - EVENT Update Unit" true true (struct :`G` 0.66 :`B` 1.0 :`A` 1.0) 3.0))
        (:`else`)))
    (:`then_1`
      (set `self.WeaponData` WeaponData))
    (:`then_2`
      (bind _as_bp_hud_gameplay (`self.As BP_HUD_Gameplay`)
        (:`then`
          (`/Game/AIPhases/Gameplay/HUD/BP_HUD_Gameplay.UpdateWeapon` _as_bp_hud_gameplay (`self.WeaponData`)))
        (:`else`)))))

(fn `GatActorUnderCursorByChannel`
  (params (TraceChannel :type "ETraceTypeQuery Enum" :default "TraceTypeQuery1"))
  (returns (Hit :type Boolean) (HitActor :type "Actor Object Reference"))
  (bind (_bblockinghit _binitialoverlap _time _distance _location _impactpoint _normal _impactnormal _physmat _hitactor) (`GameplayStatics.BreakHitResult` (`self.GetHitResultUnderCursorByChannel` TraceChannel)))
  (return _bblockinghit _hitactor))

(fn `OnRep_As BP_Character_Unit`
  (`|ExecutionSequence`
    (:`then_0`
      (`self.bShowDebug`
        (:`then`
          (`KismetSystemLibrary.PrintString` "BP_PC_Gameplay - REPNOTIFY Unit" true true (struct :`G` 0.66 :`B` 1.0 :`A` 1.0) 3.0))
        (:`else`)))
    (:`then_1`
      (bind _asbp_hud_gameplay (cast `/Game/AIPhases/Gameplay/HUD/BP_HUD_Gameplay` (`self.GetHUD`)))
      (`/Game/AIPhases/Gameplay/HUD/BP_HUD_Gameplay.UpdateUnit` _asbp_hud_gameplay (`self.As BP_Character_Unit`)))))

(fn `UserConstructionScript`)