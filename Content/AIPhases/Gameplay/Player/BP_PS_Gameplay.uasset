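; Gameplay Player State that holds a player's unit, team, weapon data, outfit, kills and deaths.
; Update events set each variable, and all but weapon data have RepNotify functions.
; OnRep_Unit passes the unit to the BP_PC_Gameplay returned by GetPlayerController, while the other RepNotifies only cast to that controller and do nothing further.
; Events and RepNotifies print debug strings behind a ShowDebug check.
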(event `UpdateUnit`
  (params (Unit :type "/Game/AIPhases/Blueprints/Units/BP_Character_Unit Object Reference"))
  (`|ExecutionSequence`
    (:`then_0`
      (`self.bShowDebug`
        (:`then`
          (`KismetSystemLibrary.PrintString` "BP_PS_Gameplay - EVENT Update Unit" true true (struct :`G` 0.66 :`B` 1.0 :`A` 1.0) 3.0))
        (:`else`)))
    (:`then_1`
      (set `self.Unit` Unit))))

(event `UpdateTeam`
  (params (Team :type "/Game/AIPhases/Blueprints/Team/Enum/E_Team Enum" :default "NewEnumerator0"))
  (`|ExecutionSequence`
    (:`then_0`
      (`self.bShowDebug`
        (:`then`
          (`KismetSystemLibrary.PrintString` "BP_PS_Gameplay - EVENT Update Unit" true true (struct :`G` 0.66 :`B` 1.0 :`A` 1.0) 3.0))
        (:`else`)))
    (:`then_1`
      (set `self.Team` Team))))

(event `UpdateWeapon`
  (params (WeaponData :type "/Game/AIPhases/Blueprints/Weapon/Data/PDA_Weapon Object Reference"))
  (`|ExecutionSequence`
    (:`then_0`
      (`self.bShowDebug`
        (:`then`
          (`KismetSystemLibrary.PrintString` "BP_PS_Gameplay - EVENT Update Unit" true true (struct :`G` 0.66 :`B` 1.0 :`A` 1.0) 3.0))
        (:`else`)))
    (:`then_1`
      (set `self.WeaponData` WeaponData))))

(event `UpdateOutfit`
  (params (Outfit :type "SkeletalMesh Object Reference"))
  (`|ExecutionSequence`
    (:`then_0`
      (`self.bShowDebug`
        (:`then`
          (`KismetSystemLibrary.PrintString` "BP_PS_Gameplay - EVENT Update Outfit" true true (struct :`G` 0.66 :`B` 1.0 :`A` 1.0) 3.0))
        (:`else`)))
    (:`then_1`
      (set `self.Outfit` Outfit))))

(event `UpdateKills`
  (params (Kills :type Integer))
  (`|ExecutionSequence`
    (:`then_0`
      (`self.bShowDebug`
        (:`then`
          (`KismetSystemLibrary.PrintString` "BP_PS_Gameplay - EVENT Update Kiills" true true (struct :`G` 0.66 :`B` 1.0 :`A` 1.0) 3.0))
        (:`else`)))
    (:`then_1`
      (set `self.Kills` Kills))))

(event `UpdateDeaths`
  (params (Deaths :type Integer))
  (`|ExecutionSequence`
    (:`then_0`
      (`self.bShowDebug`
        (:`then`
          (`KismetSystemLibrary.PrintString` "BP_PS_Gameplay - EVENT Update Deaths" true true (struct :`G` 0.66 :`B` 1.0 :`A` 1.0) 3.0))
        (:`else`)))
    (:`then_1`
      (set `self.Deaths` Deaths))))

(fn `OnRep_Deaths`
  (`|ExecutionSequence`
    (:`then_0`
      (`self.bShowDebug`
        (:`then`
          (`KismetSystemLibrary.PrintString` "BP_Character_Unit - REPNOTIFY Deaths" true true (struct :`G` 0.66 :`B` 1.0 :`A` 1.0) 3.0))
        (:`else`)))
    (:`then_1`
      (cast `/Game/AIPhases/Gameplay/Player/BP_PC_Gameplay` (`self.GetPlayerController`)))))

(fn `OnRep_Kills`
  (`|ExecutionSequence`
    (:`then_0`
      (`self.bShowDebug`
        (:`then`
          (`KismetSystemLibrary.PrintString` "BP_Character_Unit - REPNOTIFY Kills" true true (struct :`G` 0.66 :`B` 1.0 :`A` 1.0) 3.0))
        (:`else`)))
    (:`then_1`
      (cast `/Game/AIPhases/Gameplay/Player/BP_PC_Gameplay` (`self.GetPlayerController`)))))

(fn `OnRep_Outfit`
  (`|ExecutionSequence`
    (:`then_0`
      (`self.bShowDebug`
        (:`then`
          (`KismetSystemLibrary.PrintString` "BP_Character_Unit - REPNOTIFY Outfit" true true (struct :`G` 0.66 :`B` 1.0 :`A` 1.0) 3.0))
        (:`else`)))
    (:`then_1`
      (cast `/Game/AIPhases/Gameplay/Player/BP_PC_Gameplay` (`self.GetPlayerController`)))))

(fn `OnRep_Team`
  (`|ExecutionSequence`
    (:`then_0`
      (`self.bShowDebug`
        (:`then`
          (`KismetSystemLibrary.PrintString` "BP_Character_Unit - REPNOTIFY Team" true true (struct :`G` 0.66 :`B` 1.0 :`A` 1.0) 3.0))
        (:`else`)))
    (:`then_1`
      (cast `/Game/AIPhases/Gameplay/Player/BP_PC_Gameplay` (`self.GetPlayerController`)))))

(fn `OnRep_Unit`
  (`|ExecutionSequence`
    (:`then_0`
      (`self.bShowDebug`
        (:`then`
          (`KismetSystemLibrary.PrintString` "BP_Character_Unit - REPNOTIFY Unit" true true (struct :`G` 0.66 :`B` 1.0 :`A` 1.0) 3.0))
        (:`else`)))
    (:`then_1`
      (bind _asbp_pc_gameplay (cast `/Game/AIPhases/Gameplay/Player/BP_PC_Gameplay` (`self.GetPlayerController`)))
      (`/Game/AIPhases/Gameplay/Player/BP_PC_Gameplay.UnitUpdate` _asbp_pc_gameplay (`self.Unit`)))))

(fn `UserConstructionScript`)