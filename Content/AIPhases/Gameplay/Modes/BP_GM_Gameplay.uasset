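; Gameplay game mode that manages bot identities, player connections, match start and AI unit lifecycle.
; BeginPlay spawns a named, armed PlayerState per bot into the GameState's GlobalSoulArray; PostLogin tracks controllers and calls MatchStart.
; UnitSpawn creates a unit and possessing AI controller for a spawn tile's PlayerState, removing it from PlayerGraveyard.
; HandleUnitDeath adds the PlayerState to that graveyard and destroys unit and controller; controller swapping only prints debug.
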(event `self.ReceiveBeginPlay`
  (`|ExecutionSequence`
    (:`then_0`
      (`self.bShowDebug`
        (:`then`
          (`KismetSystemLibrary.PrintString` "BP_GM_Gameplay - EVENT BeginPlay" true true (struct :`G` 0.66 :`B` 1.0 :`A` 1.0) 3.0))
        (:`else`)))
    (:`then_1`
      (add `self.OnCharacterDied` (`|CreateDelegate` :!event `HandleUnitDeath`)))
    (:`then_2`
      (for _ (range (`self.BotCount`))
        (bind _returnvalue (`|SpawnActorFromClass` "/Game/AIPhases/Gameplay/Player/BP_PS_Gameplay.BP_PS_Gameplay_C" (`KismetMathLibrary.MakeTransform` (0.0 0.0 0.0)) "Undefined" "MultiplyWithRoot" null null))
        (`/Game/AIPhases/Gameplay/Player/BP_PS_Gameplay.UpdateName` _returnvalue "")
        (`/Game/AIPhases/Gameplay/Player/BP_PS_Gameplay.UpdateWeapon` _returnvalue null)
        (`self.As BP GS Gameplay`
          (:`then`
            _)
          (:`else`
            (bind _asbp_gs_gameplay (cast `/Game/AIPhases/Gameplay/Modes/BP_GS_Gameplay` (`GameplayStatics.GetGameState`)))
            (set `self.As BP GS Gameplay` _asbp_gs_gameplay)))
        (`KismetArrayLibrary.Array_Add` (`/Game/AIPhases/Gameplay/Modes/BP_GS_Gameplay.GlobalSoulArray` (`self.As BP GS Gameplay`)) _returnvalue)))))

(event `self.K2_PostLogin`
  (params (NewPlayer :type "PlayerController Object Reference"))
  (`|ExecutionSequence`
    (:`then_0`
      (`self.bShowDebug`
        (:`then`
          (`KismetSystemLibrary.PrintString` "BP_GM_Gameplay - EVENT OnPostLogin" true true (struct :`G` 0.66 :`B` 1.0 :`A` 1.0) 3.0))
        (:`else`)))
    (:`then_1`
      (`KismetArrayLibrary.Array_Add` (`self.AsAllPlayerControllers`) NewPlayer)
      (if (>= (`KismetArrayLibrary.Array_Length` (`self.AsAllPlayerControllers`)) 1)
        (`self.As BP GS Gameplay`
          (:`then`
            _)
          (:`else`
            (bind _asbp_gs_gameplay (cast `/Game/AIPhases/Gameplay/Modes/BP_GS_Gameplay` (`GameplayStatics.GetGameState`)))
            (set `self.As BP GS Gameplay` _asbp_gs_gameplay)))
        (`/Game/AIPhases/Gameplay/Modes/BP_GS_Gameplay.Match Start` (`self.As BP GS Gameplay`))))))

(event `UnitSpawn`
  (params (SpawnTile :type "Actor Object Reference"))
  (`|ExecutionSequence`
    (:`then_0`
      (`self.bShowDebug`
        (:`then`
          (`KismetSystemLibrary.PrintString` "BP_GM_Gameplay - EVENT Unit Death" true true (struct :`G` 0.66 :`B` 1.0 :`A` 1.0) 3.0))
        (:`else`)))
    (:`then_1`
      (bind _asbp_actor_spawn_tile (cast `/Game/AIPhases/Blueprints/SpawnTile/BP_Actor_SpawnTile` SpawnTile))
      (bind _playerstate (`/Game/AIPhases/Blueprints/SpawnTile/BP_Actor_SpawnTile.PlayerState` _asbp_actor_spawn_tile)
        (:`then`
          (bind _returnvalue (`|SpawnActorFromClass` "/Game/AIPhases/Blueprints/Units/BP_Character_Unit.BP_Character_Unit_C" (`self.GetTransform` _playerstate) "Undefined" "MultiplyWithRoot" null null null))
          (bind _returnvalue_2 (`|SpawnActorFromClass` "/Game/AIPhases/Blueprints/Units/AI/BP_AIController_Gameplay.BP_AIController_Gameplay_C" (`self.GetTransform` _returnvalue) "Undefined" "MultiplyWithRoot" null null))
          (`Controller.Possess` _returnvalue_2 _returnvalue)
          (`KismetArrayLibrary.Array_RemoveItem` (`self.PlayerGraveyard`) _playerstate))
        (:`else`)))))

(event `self.K2_OnLogout`
  (params (ExitingController :type "Controller Object Reference"))
  (`|ExecutionSequence`
    (:`then_0`
      (`self.bShowDebug`
        (:`then`
          (`KismetSystemLibrary.PrintString` "BP_GM_Gameplay - EVENT OnLogout" true true (struct :`G` 0.66 :`B` 1.0 :`A` 1.0) 3.0))
        (:`else`)))
    (:`then_1`
      (bind _asplayer_controller (cast `PlayerController` ExitingController))
      (`KismetArrayLibrary.Array_RemoveItem` (`self.AsAllPlayerControllers`) _asplayer_controller))))

(event `HandleUnitDeath` :!signature `self.OnCharacterDied`
  (params (Unit :type "Character Object Reference"))
  (bind _returnvalue (`Pawn.GetController` Unit))
  (`|ExecutionSequence`
    (:`then_0`
      (`self.bShowDebug`
        (:`then`
          (`KismetSystemLibrary.PrintString` "BP_GM_Gameplay - EVENT Unit Spawn" true true (struct :`G` 0.66 :`B` 1.0 :`A` 1.0) 3.0))
        (:`else`)))
    (:`then_1`
      (`KismetArrayLibrary.Array_AddUnique` (`self.PlayerGraveyard`) (`Controller.PlayerState` _returnvalue))
      (`Controller.UnPossess` _returnvalue)
      (`self.K2_DestroyActor` _returnvalue)
      (`self.K2_DestroyActor` Unit))))

(event `self.K2_OnSwapPlayerControllers`
  (params (OldPC :type "PlayerController Object Reference") (NewPC :type "PlayerController Object Reference"))
  (`|ExecutionSequence`
    (:`then_0`
      (`self.bShowDebug`
        (:`then`
          (`KismetSystemLibrary.PrintString` "BP_GM_Gameplay - EVENT OnSwap Player Controller" true true (struct :`G` 0.66 :`B` 1.0 :`A` 1.0) 3.0))
        (:`else`)))))

(fn `UserConstructionScript`)