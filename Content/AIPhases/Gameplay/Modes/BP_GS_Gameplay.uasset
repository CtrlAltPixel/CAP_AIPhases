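; Gameplay game state for a turn-based, phased match, defining match, turn, phase and action events that are mostly debug-print stubs.
; TurnStart increments TurnCount, while TurnCount and Phase rep-notifies broadcast change events; score and soul notifies are empty.
; PhaseStart clears the unit queue and starts actions, but queue filling and action spawning are unwired.
; ActionEnd pops the queue, then starts another action or ends phase and turn.
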(event `self.ReceiveBeginPlay`
  (`|ExecutionSequence`
    (:`then_0`
      (`self.bShowDebug`
        (:`then`
          (`KismetSystemLibrary.PrintString` "BP_GS_Gameplay - EVENT Begin Play" true true (struct :`G` 0.66 :`B` 1.0 :`A` 1.0) 3.0))
        (:`else`)))))

(event `Match Start`
  (`|ExecutionSequence`
    (:`then_0`
      (`self.bShowDebug`
        (:`then`
          (`KismetSystemLibrary.PrintString` "BP_Gs_Gameplay - EVENT Match Start" true true (struct :`G` 0.66 :`B` 1.0 :`A` 1.0) 3.0))
        (:`else`)))))

(event `MatchEnd`
  (`|ExecutionSequence`
    (:`then_0`
      (`self.bShowDebug`
        (:`then`
          (`KismetSystemLibrary.PrintString` "BP_Gs_Gameplay - EVENT Match End" true true (struct :`G` 0.66 :`B` 1.0 :`A` 1.0) 3.0))
        (:`else`)))))

(event `Turn Start`
  (`|ExecutionSequence`
    (:`then_0`
      (`self.bShowDebug`
        (:`then`
          (`KismetSystemLibrary.PrintString` "BP_GS_Gameplay - EVENT Turn Start" true true (struct :`G` 0.66 :`B` 1.0 :`A` 1.0) 3.0))
        (:`else`)))
    (:`then_1`
      (set `self.TurnCount` (+ (`self.TurnCount`) 1)))))

(event `TurnEnd`
  (`|ExecutionSequence`
    (:`then_0`
      (`self.bShowDebug`
        (:`then`
          (`KismetSystemLibrary.PrintString` "BP_GS_Gameplay - EVENT Turn End" true true (struct :`G` 0.66 :`B` 1.0 :`A` 1.0) 3.0))
        (:`else`)))))

(event `PhaseStart`
  (`|ExecutionSequence`
    (:`then_0`
      (`self.bShowDebug`
        (:`then`
          (`KismetSystemLibrary.PrintString` "BP_GS_Gameplay - EVENT PhaseStart" true true (struct :`G` 0.66 :`B` 1.0 :`A` 1.0) 3.0))
        (:`else`)))
    (:`then_1`
      (`KismetArrayLibrary.Array_Clear` (`self.UnitQue`))
      (bind _outactors (`GameplayStatics.GetAllActorsOfClass` "/Game/AIPhases/Blueprints/Units/BP_Character_Unit.BP_Character_Unit_C"))
      (for _array_element _outactors
        (cast `/Game/AIPhases/Blueprints/Units/AI/BP_AIController_Gameplay` (`AIBlueprintHelperLibrary.GetAIController` _array_element))
        (switch `/Game/AIPhases/Blueprints/Turns/Enums/E_Phase` (`self.Phase`)))
      (`self.ActionStart`))))

(event `PhaseEnd`
  (`|ExecutionSequence`
    (:`then_0`
      (`self.bShowDebug`
        (:`then`
          (`KismetSystemLibrary.PrintString` "BP_GS_Gameplay - EVENT Phase End" true true (struct :`G` 0.66 :`B` 1.0 :`A` 1.0) 3.0))
        (:`else`)))
    (:`then_1`
      (`self.TurnEnd`))))

(event `Planningstart`
  (`|ExecutionSequence`
    (:`then_0`
      (`self.bShowDebug`
        (:`then`
          (`KismetSystemLibrary.PrintString` "BP_GS_Gameplay - EVENT Planning Start" true true (struct :`G` 0.66 :`B` 1.0 :`A` 1.0) 3.0))
        (:`else`)))))

(event `SpellsStart`
  (`|ExecutionSequence`
    (:`then_0`
      (`self.bShowDebug`
        (:`then`
          (`KismetSystemLibrary.PrintString` "BP_GS_Gameplay - EVENT Spells Start" true true (struct :`G` 0.66 :`B` 1.0 :`A` 1.0) 3.0))
        (:`else`)))))

(event `PreperationStart`
  (`|ExecutionSequence`
    (:`then_0`
      (`self.bShowDebug`
        (:`then`
          (`KismetSystemLibrary.PrintString` "BP_GS_Gameplay - EVENT Preperation Start" true true (struct :`G` 0.66 :`B` 1.0 :`A` 1.0) 3.0))
        (:`else`)))))

(event `DashStart`
  (`|ExecutionSequence`
    (:`then_0`
      (`self.bShowDebug`
        (:`then`
          (`KismetSystemLibrary.PrintString` "BP_GS_Gameplay - EVENT Dash Start" true true (struct :`G` 0.66 :`B` 1.0 :`A` 1.0) 3.0))
        (:`else`)))))

(event `CombatStart`
  (`|ExecutionSequence`
    (:`then_0`
      (`self.bShowDebug`
        (:`then`
          (`KismetSystemLibrary.PrintString` "BP_GS_Gameplay - EVENT Combat Start" true true (struct :`G` 0.66 :`B` 1.0 :`A` 1.0) 3.0))
        (:`else`)))))

(event `DeathStart`
  (`|ExecutionSequence`
    (:`then_0`
      (`self.bShowDebug`
        (:`then`
          (`KismetSystemLibrary.PrintString` "BP_GS_Gameplay - EVENT Death Start" true true (struct :`G` 0.66 :`B` 1.0 :`A` 1.0) 3.0))
        (:`else`)))))

(event `MovementStart`
  (`|ExecutionSequence`
    (:`then_0`
      (`self.bShowDebug`
        (:`then`
          (`KismetSystemLibrary.PrintString` "BP_GS_Gameplay - EVENT MovementStart" true true (struct :`G` 0.66 :`B` 1.0 :`A` 1.0) 3.0))
        (:`else`)))))

(event `ReSpawnStart`
  (`|ExecutionSequence`
    (:`then_0`
      (`self.bShowDebug`
        (:`then`
          (`KismetSystemLibrary.PrintString` "BP_GS_Gameplay - EVENT Spawn Start" true true (struct :`G` 0.66 :`B` 1.0 :`A` 1.0) 3.0))
        (:`else`)))))

(event `ActionStart`
  (`|ExecutionSequence`
    (:`then_0`
      (`self.bShowDebug`
        (:`then`
          (`KismetSystemLibrary.PrintString` "BP_GS_Gameplay - EVENT Action Start" true true (struct :`G` 0.66 :`B` 1.0 :`A` 1.0) 3.0))
        (:`else`)))))

(event `HandleAction`
  (params (Action :type "/Game/AIPhases/Blueprints/Action/BP_Actor_Action Object Reference"))
  (`|ExecutionSequence`
    (:`then_0`
      (`self.bShowDebug`
        (:`then`
          (`KismetSystemLibrary.PrintString` "BP_GS_Gameplay - EVENT Phase End" true true (struct :`G` 0.66 :`B` 1.0 :`A` 1.0) 3.0))
        (:`else`)))
    (:`then_1`
      (`self.K2_DestroyActor` Action))))

(event `ActionEnd`
  (`|ExecutionSequence`
    (:`then_0`
      (`self.bShowDebug`
        (:`then`
          (`KismetSystemLibrary.PrintString` "BP_GS_Gameplay - EVENT Phase End" true true (struct :`G` 0.66 :`B` 1.0 :`A` 1.0) 3.0))
        (:`else`)))
    (:`then_1`
      (`KismetArrayLibrary.Array_Remove` (`self.UnitQue`))
      (if (`KismetArrayLibrary.Array_IsEmpty` (`self.UnitQue`))
        (`self.PhaseEnd`)
        (else
          (`self.ActionStart`))))))

(fn `OnRep_BlueTeamScore`)

(fn `OnRep_GlobalSoulArray`)

(fn `OnRep_Phase`
  (`self.OnPhaseChange` (`self.Phase`)))

(fn `OnRep_RedTeamScore`)

(fn `OnRep_TurnCount`
  (`|ExecutionSequence`
    (:`then_0`
      (`self.bShowDebug`
        (:`then`
          (`KismetSystemLibrary.PrintString` "BP_GS_Gameplay - EVENT Turn Start" true true (struct :`G` 0.66 :`B` 1.0 :`A` 1.0) 3.0))
        (:`else`)))
    (:`then_1`
      (`self.OnTurnChange` (`self.TurnCount`)))))

(fn `UserConstructionScript`)