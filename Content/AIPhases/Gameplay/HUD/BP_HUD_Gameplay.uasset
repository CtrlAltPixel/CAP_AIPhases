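; Gameplay HUD Blueprint that owns the WB_HUD_Gameplay widget and relays unit and weapon changes to it.
; BeginPlay creates the widget if none is valid and adds it to the viewport, with a redundant second AddToViewport call after creation.
; UpdateUnit and UpdateWeapon store the incoming data and forward it to the widget.
; Each event can print a debug message gated by ShowDebug, though UpdateWeapon's message is mislabeled as Update Unit.
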(event `self.ReceiveBeginPlay`
  (`|ExecutionSequence`
    (:`then_0`
      (`self.bShowDebug`
        (:`then`
          (`KismetSystemLibrary.PrintString` "BP_HUD_Gameplay - EVENT Begin Play" true true (struct :`G` 0.66 :`B` 1.0 :`A` 1.0) 3.0))
        (:`else`)))
    (:`then_1`
      (`self.AsWBHUDAIPhases`
        (:`then`
          _)
        (:`else`
          (bind _returnvalue (`|CreateWidget` "/Game/AIPhases/Gameplay/HUD/UI/WB_HUD_Gameplay.WB_HUD_Gameplay_C"))
          (bind _output_get (set `self.AsWBHUDAIPhases` _returnvalue))
          (`UserWidget.AddToViewport` _output_get 0)))
      (`UserWidget.AddToViewport` (`self.AsWBHUDAIPhases`) 0))))

(event `UpdateUnit`
  (params (Unit :type "/Game/AIPhases/Blueprints/Units/BP_Character_Unit Object Reference"))
  (`|ExecutionSequence`
    (:`then_0`
      (`self.bShowDebug`
        (:`then`
          (`KismetSystemLibrary.PrintString` "BP_HUD_Gameplay - EVENT Update Unit" true true (struct :`G` 0.66 :`B` 1.0 :`A` 1.0) 3.0))
        (:`else`)))
    (:`then_1`
      (set `self.Unit` Unit)
      (`/Game/AIPhases/Gameplay/HUD/UI/WB_HUD_Gameplay.UpdateUnit` (`self.AsWBHUDAIPhases`) (`self.Unit`)))))

(event `UpdateWeapon`
  (params (WeaponData :type "/Game/AIPhases/Blueprints/Weapon/Data/PDA_Weapon Object Reference"))
  (`|ExecutionSequence`
    (:`then_0`
      (`self.bShowDebug`
        (:`then`
          (`KismetSystemLibrary.PrintString` "BP_HUD_Gameplay - EVENT Update Unit" true true (struct :`G` 0.66 :`B` 1.0 :`A` 1.0) 3.0))
        (:`else`)))
    (:`then_1`
      (set `self.WeaponData` WeaponData)
      (`/Game/AIPhases/Gameplay/HUD/UI/WB_HUD_Gameplay.UpdateWeapon` (`self.AsWBHUDAIPhases`) (`self.WeaponData`)))))

(fn `UserConstructionScript`)