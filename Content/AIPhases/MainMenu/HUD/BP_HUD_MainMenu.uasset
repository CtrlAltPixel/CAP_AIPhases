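; BP_HUD_MainMenu is the HUD for the main menu, putting the menu widget on screen when play begins.
; BeginPlay creates WBP_HUD_MainMenu for the owning player controller if none is stored, then adds it to the viewport.
; It then switches that controller to UI-only input focused on the widget, after an optional debug print.
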(event `self.ReceiveBeginPlay`
  (`|ExecutionSequence`
    (:`then_0`
      (`self.bShowDebug`
        (:`then`
          (`KismetSystemLibrary.PrintString` "BP_HUD_MainMenu - EVENT Begin Play" true true (struct :`G` 0.66 :`B` 1.0 :`A` 1.0) 3.0))
        (:`else`)))
    (:`then_1`
      (`self.As WBP_HUD_MainMenu`
        (:`then`
          _)
        (:`else`
          (bind _returnvalue (`|CreateWidget` "/Game/AIPhases/MainMenu/HUD/UI/WBP_HUD_MainMenu.WBP_HUD_MainMenu_C" (`self.GetOwningPlayerController`)))
          (set `self.As WBP_HUD_MainMenu` _returnvalue)))
      (`UserWidget.AddToViewport` (`self.As WBP_HUD_MainMenu`) 0))
    (:`then_2`
      (`WidgetBlueprintLibrary.SetInputMode_UIOnlyEx` (`self.GetOwningPlayerController`) (`self.As WBP_HUD_MainMenu`)))))

(fn `UserConstructionScript`)